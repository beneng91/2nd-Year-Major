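; BP_LaserBeam is a laser hazard that kills and respawns any PhysicsPlayer it hits.
; Each tick it line-traces forward on the Camera channel, sets the beam particle's end point and shows an impact effect on blocking hits.
; Beam length snaps back to the hit distance and grows over time up to a cap, so it extends gradually when unblocked.
; Player hits spawn death particles and sound before calling RespawnPlayer.
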(event EventBeginPlay
  ;[1 1 1] Colour
  (Effects|Components|ParticleSystem|SetColorParameter (Variables|Default|GetLaserBeam) "Color" "(R=1.000000,G=0.030093,B=0.010197,A=1.000000)")
  (Effects|Components|ParticleSystem|SetColorParameter (Variables|Default|GetLaserImpact) "Color" "(R=0.055236,G=1.000000,B=0.121617,A=1.000000)"))

(event EventTick
  (params (DeltaSeconds :type Float%20%28single-precision%29))
  (bind _returnvalue (Transformation|GetActorLocation))
  (Variables|Default|SetDelta%20Seconds DeltaSeconds)
  (Utilities|FlowControl|Sequence
    (:then_0
      ;[1 1 1] Raycast Logic
      (Variables|Default|SetTrace%20End (+ _returnvalue (* (Transformation|GetActorForwardVector) (Variables|Default|GetDistance))))
      (bind _outhit (Collision|LineTraceByChannel _returnvalue (+ _returnvalue (* (Transformation|GetActorForwardVector) (Variables|Default|GetDistance))) "TraceTypeQuery2" false 0 "None"))
      (Variables|Default|SetBlockHit (.bBlockingHit (Collision|BreakHitResult _outhit)))
      (Variables|Default|SetHit%20Location (.Location (Collision|BreakHitResult _outhit)))
      (Variables|Default|SetActorHit (.HitActor (Collision|BreakHitResult _outhit)))
      ;[1 1 1] Impact Logic
      (Effects|Components|ParticleSystem|SetVectorParameter (Variables|Default|GetLaserBeam) "LaserEnd" (select (Variables|Default|GetBlockHit) (Variables|Default|GetHit%20Location) (Variables|Default|GetTrace%20End)))
      (Rendering|SetVisibility (Variables|Default|GetLaserImpact) (Variables|Default|GetBlockHit) false)
      (Transformation|SetWorldLocation (Variables|Default|GetLaserImpact) (Variables|Default|GetHit%20Location) false false)
      (if (Variables|Default|GetBlockHit)
        (Variables|Default|SetDistance (Math|Vector|VectorLength (- (Variables|Default|GetHit%20Location) (Transformation|GetActorLocation))))))
    (:then_1
      ;[1 1 1] Speed of Laser
      (if (< (Variables|Default|GetDistance) 5e+03)
        (Variables|Default|SetDistance (+ (Variables|Default|GetDistance) (* (Variables|Default|GetDelta%20Seconds) 2e+03)))))
    (:then_2
      ;[1 1 1] Player death logic
      (bind _asphysics_player (Utilities|Casting|CastToPhysicsPlayer (Variables|Default|GetActorHit)))
      (Variables|Default|SetPlayer%20REF _asphysics_player)
      (Effects|SpawnEmitteratLocation "/Game/Particles/P_Player_Death.P_Player_Death" (Variables|Default|GetHit%20Location))
      (Audio|PlaySound2D "/Game/Audio/SFX/Player_Spawn/Player_Despawn_Cue.Player_Despawn_Cue" 1.0 1.0 0.0 0 0)
      (Class|PhysicsCharacterSC|RespawnPlayer (Variables|/Game/Prototype/Liam/PhysicsPlayer.PhysicsPlayer_C|GetPhysicsCharacterSC (Variables|Default|GetPlayer%20REF)) (Variables|/Game/GameManagerBP.GameManagerBP_C|GetGameManager (Variables|/Game/Prototype/Liam/PhysicsPlayer.PhysicsPlayer_C|GetGame%20Manager (Variables|Default|GetPlayer%20REF))) (Variables|/Game/Prototype/Liam/PhysicsPlayer.PhysicsPlayer_C|GetRespawn%20Delay (Variables|Default|GetPlayer%20REF))))))

(fn ConstructionScript)
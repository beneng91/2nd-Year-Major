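; SaberBP is a prototype lightsaber that sparks on contact, clashes with other sabers and respawns players it hits.
; Tick traces from blade base to tip, spawning spark and burn effects at hits.
; Saber overlaps launch the wielding Test character away with a clash effect, gated by a delayed-reset DoOnce.
; Capsule overlaps respawn the cached TestPlayer with a death effect, or only cache the character when none is valid.
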(event OnComponentEndOverlap(SaberOverlap)
  (params (OverlappedComponent :type Primitive%20Component%20Object%20Reference) (OtherActor :type Actor%20Object%20Reference) (OtherComp :type Primitive%20Component%20Object%20Reference) (OtherBodyIndex :type Integer))
  (bind _lightsaber (Variables|Default|GetLightsaber))
  (bind _returnvalue (Transformation|GetWorldLocation _lightsaber))
  (Utilities|FlowControl|Sequence
    (:then_0
      ;[1 1 1] Saber knockback on Saber
      (Utilities|FlowControl|Delay 0.5)
      (Utilities|FlowControl|DoOnce false) ; enters at Reset
    )
    (:then_1
      ;[1 1 1] Hitting players
      (Utilities|FlowControl|Delay 0.5)
      (Utilities|FlowControl|DoOnce false) ; enters at Reset
    )))

(event OnComponentBeginOverlap(SaberOverlap)
  (params (OverlappedComponent :type Primitive%20Component%20Object%20Reference) (OtherActor :type Actor%20Object%20Reference) (OtherComp :type Primitive%20Component%20Object%20Reference) (OtherBodyIndex :type Integer) (bFromSweep :type Boolean) (SweepResult :type Hit%20Result%20Structure%20%28by%20ref%29))
  (bind _lightsaber (Variables|Default|GetLightsaber))
  (bind _returnvalue (Transformation|GetWorldLocation _lightsaber))
  (Utilities|FlowControl|Sequence
    (:then_0
      ;[1 1 1] Saber knockback on Saber
      (Utilities|Casting|CastToSaberBP OtherActor)
      (Utilities|FlowControl|DoOnce false
        (:Completed
          (bind _astest (Utilities|Casting|CastToTest (Actor|GetAttachParentActor)))
          (Niagara|SpawnSystematLocation "/Game/Prototype/BenTesting/LightSaber/NE_SaberClash_System.NE_SaberClash_System" _returnvalue)
          (Character|LaunchCharacter _astest (* (Math|Vector|MakeVector (.x (Math|Vector|Normalize (Math|Vector|MakeVector (.x (Math|Vector|GetUnitDirection(Vector) _returnvalue (Transformation|GetActorLocation _astest))) (.y (Math|Vector|GetUnitDirection(Vector) _returnvalue (Transformation|GetActorLocation _astest))) 0.0))) (.y (Math|Vector|Normalize (Math|Vector|MakeVector (.x (Math|Vector|GetUnitDirection(Vector) _returnvalue (Transformation|GetActorLocation _astest))) (.y (Math|Vector|GetUnitDirection(Vector) _returnvalue (Transformation|GetActorLocation _astest))) 0.0))) (Variables|Default|GetLaunch%20Angle)) (Variables|Default|GetLaunch%20Velocity)) false false)
          (Development|PrintString "Hit the sword"))))
    (:then_1
      ;[1 1 1] Hitting players
      (Utilities|Casting|CastToCapsuleComponent OtherComp)
      (Utilities|IsValid (Variables|Default|GetTest%20Player)
        (:Is%20Valid
          (Niagara|SpawnSystematLocation "/Game/Prototype/BenTesting/LightSaber/Playerdeath.Playerdeath" (Transformation|GetWorldLocation (Variables|/Game/SideScrollerCPP/Blueprints/Test.Test_C|GetCenter (Variables|Default|GetTest%20Player))))
          (Class|QuantumCollapseCharacter|RespawnPlayer (Variables|Default|GetTest%20Player) (Variables|/Game/SideScrollerCPP/Blueprints/Test.Test_C|GetSpawnPos (Variables|Default|GetTest%20Player)))
          (Development|PrintString "I hit the player"))
        (:Is%20Not%20Valid
          (Development|PrintString "Not Valid")
          (bind _astest_2 (Utilities|Casting|CastToTest OtherActor))
          (Variables|Default|SetTest%20Player _astest_2))))))

(event EventTick
  (params (DeltaSeconds :type Float%20%28single-precision%29))
  (bind _returnvalue (Math|Random|RandomFloatinRange 0.5 0.9))
  (bind _lightsaber (Variables|Default|GetLightsaber))
  (bind _returnvalue_2 (Math|Conversions|ToVector(Float) _returnvalue))
  ;[1 1 1] Saber Sparks
  (Utilities|FlowControl|Sequence
    (:then_0
      (bind (_outhit _returnvalue_3) (Collision|LineTraceByChannel (Transformation|GetSocketLocation _lightsaber "Base") (Transformation|GetSocketLocation _lightsaber "Tip") "TraceTypeQuery1" false 0 "None" true "(R=1.000000,G=0.000000,B=0.000000,A=1.000000)" "(R=0.000000,G=1.000000,B=0.000000,A=1.000000)" 0.5))
      (if _returnvalue_3
        (Niagara|SpawnSystematLocation "/Game/Prototype/BenTesting/LightSaber/NE_SaberSparks_System.NE_SaberSparks_System" (.Location (Collision|BreakHitResult _outhit)) "0, 0, 0" _returnvalue_2)
        (Niagara|SpawnSystematLocation "/Game/Prototype/BenTesting/LightSaber/NE_SaberBurn_System.NE_SaberBurn_System" (.Location (Collision|BreakHitResult _outhit)) "0, 0, 0" _returnvalue_2)))))

(fn ConstructionScript)
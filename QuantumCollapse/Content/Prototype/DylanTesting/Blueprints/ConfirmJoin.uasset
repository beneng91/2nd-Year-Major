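; ConfirmJoin is a prototype Blueprint that populates what appears to be character select with players.
; Its Joining event spawns a CS_Player at every PlayerStart, numbers its outline, and registers it in CS_GameStateBase's player list.
; Each player gets the skin mesh and material at its loop index from NewGameInstance's arrays.
; The loop overwrites the game instance's player count and mesh/material selection each pass, so only the final values remain.
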(event Custom|Joining
  (bind _asnew_game_instance (Utilities|Casting|CastToNewGameInstance (Game|GetGameInstance)))
  (bind _ascs_game_state_base (Utilities|Casting|CastToCS_GameStateBase (Game|GetGameState)))
  (bind _outactors (Actor|GetAllActorsOfClass "/Script/Engine.PlayerStart"))
  (bind _output_get (Variables|Default|SetPlayerStartArray _outactors))
  (for (_array_element _array_index) _output_get
    (bind _returnvalue (Game|SpawnActorfromClass "/Game/Prototype/Liam/CS_Player.CS_Player_C" (Transformation|GetActorTransform _array_element) "Undefined" 0 (+ _array_index 1) 0))
    (Utilities|Array|AddUnique (Variables|/Game/Blueprints/CS_GameStateBase.CS_GameStateBase_C|GetCS_PlayerList _ascs_game_state_base) _returnvalue)
    (Variables|/Game/SideScrollerCPP/Blueprints/NewGameInstance.NewGameInstance_C|SetPlayerNumbers _asnew_game_instance (+ _array_index 1))
    (Variables|/Game/SideScrollerCPP/Blueprints/NewGameInstance.NewGameInstance_C|SetCharacterSelectMesh _asnew_game_instance _array_index)
    (Variables|/Game/SideScrollerCPP/Blueprints/NewGameInstance.NewGameInstance_C|SetCharacterSelectMaterial _asnew_game_instance _array_index)
    (Rendering|Material|SetMaterial (Variables|/Game/Prototype/Liam/CS_Player.CS_Player_C|GetSkeletalMesh _returnvalue) 0 (Utilities|Array|Get(acopy) (Variables|/Game/SideScrollerCPP/Blueprints/NewGameInstance.NewGameInstance_C|GetMaterialInstanceArray _asnew_game_instance) _array_index))
    (Class|SkinnedMeshComponent|SetSkeletalMesh (Variables|/Game/Prototype/Liam/CS_Player.CS_Player_C|GetSkeletalMesh _returnvalue) (Utilities|Array|Get(acopy) (Variables|/Game/SideScrollerCPP/Blueprints/NewGameInstance.NewGameInstance_C|GetCharacterSkinArray _asnew_game_instance) _array_index) true)))

(fn ConstructionScript)
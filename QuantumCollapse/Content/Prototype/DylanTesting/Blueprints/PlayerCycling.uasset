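; PlayerCycling is a prototype Blueprint that spawns the players set up at character select when play begins.
; It gathers all PlayerStarts, then loops over the character-select meshes stored in NewGameInstance, spawning a PhysicsPlayer at the start with the matching index.
; Each spawned player receives its mesh and material through WinningPlayerChanges.
; An unconnected validity check with a debug print never runs.
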(event EventBeginPlay
  (bind _outactors (Actor|GetAllActorsOfClass "/Script/Engine.PlayerStart"))
  (bind _output_get (Variables|Default|Setplayerstarts _outactors))
  (bind _asnew_game_instance (Utilities|Casting|CastToNewGameInstance (Game|GetGameInstance)))
  (Variables|Default|SetGameInstance _asnew_game_instance)
  (for (_ _array_index) (Variables|/Game/SideScrollerCPP/Blueprints/NewGameInstance.NewGameInstance_C|GetCharacterSelectMeshes (Variables|Default|GetGameInstance))
    (if true
      (bind _returnvalue (Game|SpawnActorfromClass "/Game/Prototype/Liam/PhysicsPlayer.PhysicsPlayer_C" (Transformation|GetActorTransform (Utilities|Array|Get(acopy) _output_get _array_index)) "Undefined" 0 0 0))
      (Variables|Default|SetNewVar_0 _returnvalue)
      (Default|WinningPlayerChanges (Variables|Default|GetNewVar_0) (Utilities|Array|Get(acopy) (Variables|/Game/SideScrollerCPP/Blueprints/NewGameInstance.NewGameInstance_C|GetCharacterSelectMeshes (Variables|Default|GetGameInstance)) _array_index) (Utilities|Array|Get(acopy) (Variables|/Game/SideScrollerCPP/Blueprints/NewGameInstance.NewGameInstance_C|GetCharacterSelectMaterials (Variables|Default|GetGameInstance)) _array_index)))))

(fn ConstructionScript)
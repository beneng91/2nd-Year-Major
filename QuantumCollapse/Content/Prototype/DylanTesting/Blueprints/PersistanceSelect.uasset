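; Prototype level actor that carries players' character-select choices into the match, applying saved meshes and materials before the game begins.
; On BeginPlay, SaveMeshAndMaterials loops PhysicsPlayer actors up to MaxPlayerCount, reading each index's mesh and material picks from NewGameInstance.
; The mesh index picks one of four per-character material arrays for WinningPlayerChanges, then GameManagerBP's Start is called.
; Older backup and disconnected spawn variants remain, alongside a random PlayerStart location helper.
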(event Custom|CustomEvent
  ;[1 1 1] backup
  (bind _outactors (Actor|GetAllActorsOfClass "/Script/Engine.PlayerStart"))
  (Variables|Default|Setplayerstartarray _outactors)
  (bind _asnew_game_instance (Utilities|Casting|CastToNewGameInstance (Game|GetGameInstance)))
  (for (_array_element _array_index) (Variables|/Game/SideScrollerCPP/Blueprints/NewGameInstance.NewGameInstance_C|GetCharacterSelectMeshes _asnew_game_instance)
    (if (< _array_index (Variables|/Game/SideScrollerCPP/Blueprints/NewGameInstance.NewGameInstance_C|GetMaxPlayerCount _asnew_game_instance))
      (bind _returnvalue (Actor|GetActorOfClass "/Game/GameManagerBP.GameManagerBP_C"))
      (Default|WinningPlayerChanges (Utilities|Array|Get(acopy) (Variables|/Game/GameManagerBP.GameManagerBP_C|GetPlayerArray _returnvalue) _array_index) _array_element (Utilities|Select :Index (Variables|/Game/SideScrollerCPP/Blueprints/NewGameInstance.NewGameInstance_C|GetCharacterSelectMesh _asnew_game_instance) :Option%200 (Utilities|Array|Get(acopy) (Variables|/Game/SideScrollerCPP/Blueprints/NewGameInstance.NewGameInstance_C|GetCharacterSelectMaterials1 _asnew_game_instance) (Utilities|Array|Get(acopy) (Variables|/Game/SideScrollerCPP/Blueprints/NewGameInstance.NewGameInstance_C|GetPlayerSelectedMaterialByInt _asnew_game_instance) _array_index)) :Option%201 (Utilities|Array|Get(acopy) (Variables|/Game/SideScrollerCPP/Blueprints/NewGameInstance.NewGameInstance_C|GetOtterMaterialsArray _asnew_game_instance) (Utilities|Array|Get(acopy) (Variables|/Game/SideScrollerCPP/Blueprints/NewGameInstance.NewGameInstance_C|GetPlayerSelectedMaterialByInt _asnew_game_instance) _array_index)) :Option%202 (Utilities|Array|Get(acopy) (Variables|/Game/SideScrollerCPP/Blueprints/NewGameInstance.NewGameInstance_C|GetRobotMaterialsArray _asnew_game_instance) (Utilities|Array|Get(acopy) (Variables|/Game/SideScrollerCPP/Blueprints/NewGameInstance.NewGameInstance_C|GetPlayerSelectedMaterialByInt _asnew_game_instance) _array_index)) :Option%203 (Utilities|Array|Get(acopy) (Variables|/Game/SideScrollerCPP/Blueprints/NewGameInstance.NewGameInstance_C|GetSinisterMaterialsArray _asnew_game_instance) (Utilities|Array|Get(acopy) (Variables|/Game/SideScrollerCPP/Blueprints/NewGameInstance.NewGameInstance_C|GetPlayerSelectedMaterialByInt _asnew_game_instance) _array_index))))))
  (Development|PrintString "Complete")
  (bind _returnvalue_2 (Actor|GetActorOfClass "/Game/GameManagerBP.GameManagerBP_C"))
  (Default|Start _returnvalue_2))

(event Custom|event
  (bind _outactors (Actor|GetAllActorsOfClass "/Script/Engine.PlayerStart"))
  (Variables|Default|Setplayerstartarray _outactors)
  (bind _asnew_game_instance (Utilities|Casting|CastToNewGameInstance (Game|GetGameInstance)))
  (for (_array_element _array_index) (Variables|/Game/SideScrollerCPP/Blueprints/NewGameInstance.NewGameInstance_C|GetCharacterSelectMeshes _asnew_game_instance)
    (if (< _array_index (Variables|/Game/SideScrollerCPP/Blueprints/NewGameInstance.NewGameInstance_C|GetMaxPlayerCount _asnew_game_instance))
      (bind _returnvalue (Actor|GetActorOfClass "/Game/GameManagerBP.GameManagerBP_C"))
      (Default|WinningPlayerChanges (Utilities|Array|Get(acopy) (Variables|/Game/GameManagerBP.GameManagerBP_C|GetPlayerArray _returnvalue) _array_index) _array_element (Utilities|Select :Index (Variables|/Game/SideScrollerCPP/Blueprints/NewGameInstance.NewGameInstance_C|GetCharacterSelectMesh _asnew_game_instance) :Option%200 (Utilities|Array|Get(acopy) (Variables|/Game/SideScrollerCPP/Blueprints/NewGameInstance.NewGameInstance_C|GetCharacterSelectMaterials1 _asnew_game_instance) (Utilities|Array|Get(acopy) (Variables|/Game/SideScrollerCPP/Blueprints/NewGameInstance.NewGameInstance_C|GetPlayerSelectedMaterialByInt _asnew_game_instance) _array_index)) :Option%201 (Utilities|Array|Get(acopy) (Variables|/Game/SideScrollerCPP/Blueprints/NewGameInstance.NewGameInstance_C|GetOtterMaterialsArray _asnew_game_instance) (Utilities|Array|Get(acopy) (Variables|/Game/SideScrollerCPP/Blueprints/NewGameInstance.NewGameInstance_C|GetPlayerSelectedMaterialByInt _asnew_game_instance) _array_index)) :Option%202 (Utilities|Array|Get(acopy) (Variables|/Game/SideScrollerCPP/Blueprints/NewGameInstance.NewGameInstance_C|GetRobotMaterialsArray _asnew_game_instance) (Utilities|Array|Get(acopy) (Variables|/Game/SideScrollerCPP/Blueprints/NewGameInstance.NewGameInstance_C|GetPlayerSelectedMaterialByInt _asnew_game_instance) _array_index)) :Option%203 (Utilities|Array|Get(acopy) (Variables|/Game/SideScrollerCPP/Blueprints/NewGameInstance.NewGameInstance_C|GetSinisterMaterialsArray _asnew_game_instance) (Utilities|Array|Get(acopy) (Variables|/Game/SideScrollerCPP/Blueprints/NewGameInstance.NewGameInstance_C|GetPlayerSelectedMaterialByInt _asnew_game_instance) _array_index))))))
  (Development|PrintString "Complete")
  (bind _returnvalue_2 (Actor|GetActorOfClass "/Game/GameManagerBP.GameManagerBP_C"))
  (Default|Start _returnvalue_2))

(event EventBeginPlay
  (CallFunction|SaveMeshandMaterials self))

(fn ConstructionScript)

(fn SpawnLocations
  (return (Transformation|GetActorLocation (Utilities|Array|Get(acopy) (Variables|Default|Getplayerstartarray) (Math|Random|RandomIntegerinRange 0 (- (Utilities|Array|Length (Variables|Default|Getplayerstartarray)) 1))))))

(fn SetMaterialNMesh
  (params (Material :type Material%20Interface%20Object%20Reference) (NewMesh :type Skeletal%20Mesh%20Object%20Reference))
  (bind _asnew_game_instance (Utilities|Casting|CastToNewGameInstance (Game|GetGameInstance)))
  (Rendering|Material|SetMaterial (Variables|/Game/SideScrollerCPP/Blueprints/NewGameInstance.NewGameInstance_C|GetNewVar_0 _asnew_game_instance) 0 Material)
  (Class|SkinnedMeshComponent|SetSkeletalMesh (Variables|/Game/SideScrollerCPP/Blueprints/NewGameInstance.NewGameInstance_C|GetNewVar_0 _asnew_game_instance) NewMesh true))

(fn SaveMeshandMaterials
  (bind _outactors (Actor|GetAllActorsOfClass "/Script/Engine.PlayerStart"))
  (Variables|Default|Setplayerstartarray _outactors)
  (bind _asnew_game_instance (Utilities|Casting|CastToNewGameInstance (Game|GetGameInstance)))
  (bind _outactors_2 (Actor|GetAllActorsOfClass "/Game/Prototype/Liam/PhysicsPlayer.PhysicsPlayer_C"))
  (for (_array_element _array_index) _outactors_2
    (if (< _array_index (Variables|/Game/SideScrollerCPP/Blueprints/NewGameInstance.NewGameInstance_C|GetMaxPlayerCount _asnew_game_instance))
      (bind _returnvalue (Actor|GetActorOfClass "/Game/GameManagerBP.GameManagerBP_C"))
      (switch int (Utilities|Array|Get(acopy) (Variables|/Game/SideScrollerCPP/Blueprints/NewGameInstance.NewGameInstance_C|GetPlayerSelectedMeshByInt _asnew_game_instance) _array_index)
        (:Default
          (Development|PrintString "Fucked"))
        (:0
          (Default|WinningPlayerChanges _array_element (Utilities|Array|Get(acopy) (Variables|/Game/SideScrollerCPP/Blueprints/NewGameInstance.NewGameInstance_C|GetCharacterSelectMeshes _asnew_game_instance) (Utilities|Array|Get(acopy) (Variables|/Game/SideScrollerCPP/Blueprints/NewGameInstance.NewGameInstance_C|GetPlayerSelectedMeshByInt _asnew_game_instance) _array_index)) (Utilities|Array|Get(acopy) (Variables|/Game/SideScrollerCPP/Blueprints/NewGameInstance.NewGameInstance_C|GetCharacterSelectMaterials1 _asnew_game_instance) (Utilities|Array|Get(acopy) (Variables|/Game/SideScrollerCPP/Blueprints/NewGameInstance.NewGameInstance_C|GetPlayerSelectedMaterialByInt _asnew_game_instance) _array_index))))
        (:1
          (Default|WinningPlayerChanges _array_element (Utilities|Array|Get(acopy) (Variables|/Game/SideScrollerCPP/Blueprints/NewGameInstance.NewGameInstance_C|GetCharacterSelectMeshes _asnew_game_instance) (Utilities|Array|Get(acopy) (Variables|/Game/SideScrollerCPP/Blueprints/NewGameInstance.NewGameInstance_C|GetPlayerSelectedMeshByInt _asnew_game_instance) _array_index)) (Utilities|Array|Get(acopy) (Variables|/Game/SideScrollerCPP/Blueprints/NewGameInstance.NewGameInstance_C|GetOtterMaterialsArray _asnew_game_instance) (Utilities|Array|Get(acopy) (Variables|/Game/SideScrollerCPP/Blueprints/NewGameInstance.NewGameInstance_C|GetPlayerSelectedMaterialByInt _asnew_game_instance) _array_index))))
        (:2
          (Default|WinningPlayerChanges _array_element (Utilities|Array|Get(acopy) (Variables|/Game/SideScrollerCPP/Blueprints/NewGameInstance.NewGameInstance_C|GetCharacterSelectMeshes _asnew_game_instance) (Utilities|Array|Get(acopy) (Variables|/Game/SideScrollerCPP/Blueprints/NewGameInstance.NewGameInstance_C|GetPlayerSelectedMeshByInt _asnew_game_instance) _array_index)) (Utilities|Array|Get(acopy) (Variables|/Game/SideScrollerCPP/Blueprints/NewGameInstance.NewGameInstance_C|GetRobotMaterialsArray _asnew_game_instance) (Utilities|Array|Get(acopy) (Variables|/Game/SideScrollerCPP/Blueprints/NewGameInstance.NewGameInstance_C|GetPlayerSelectedMaterialByInt _asnew_game_instance) _array_index))))
        (:3
          (Default|WinningPlayerChanges _array_element (Utilities|Array|Get(acopy) (Variables|/Game/SideScrollerCPP/Blueprints/NewGameInstance.NewGameInstance_C|GetCharacterSelectMeshes _asnew_game_instance) (Utilities|Array|Get(acopy) (Variables|/Game/SideScrollerCPP/Blueprints/NewGameInstance.NewGameInstance_C|GetPlayerSelectedMeshByInt _asnew_game_instance) _array_index)) (Utilities|Array|Get(acopy) (Variables|/Game/SideScrollerCPP/Blueprints/NewGameInstance.NewGameInstance_C|GetSinisterMaterialsArray _asnew_game_instance) (Utilities|Array|Get(acopy) (Variables|/Game/SideScrollerCPP/Blueprints/NewGameInstance.NewGameInstance_C|GetPlayerSelectedMaterialByInt _asnew_game_instance) _array_index)))))))
  (Development|PrintString "Complete")
  (bind _returnvalue_2 (Actor|GetActorOfClass "/Game/GameManagerBP.GameManagerBP_C"))
  (Default|Start _returnvalue_2))
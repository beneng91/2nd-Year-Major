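; Prototype physics-driven player pawn for side-on movement in the Y-Z plane, with jumping, wall climbing, grappling and a saber lunge.
; Each Tick, line traces set collision flags that drive movement, climbing, ledge boosts and grapple release.
; PhysicsCharacterSC supplies grapple raycasts, swing force and lives, while a cable draws the rope.
; Saber input sets mesh facing, charged lunges launch the box along the saber's axis, and inputs cycle character meshes and materials.
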(event Custom|CycleLeftMesh
  ;[1 1 1] Cycling through different character meshs
  (if (<= (Variables|Default|GetmeshChoice) 0)
    (Variables|Default|SetmeshChoice 3)
    (else
      (Math|Integer|DecrementInt (Variables|Default|GetmeshChoice)
        (:%20%20
          _))))
  (CallFunction|SetMesh (Variables|Default|GetCharacterMeshArray) (Variables|Default|GetmeshChoice)))

(event Custom|CycleRightMesh
  ;[1 1 1] Cycling through different character meshs
  (if (>= (Variables|Default|GetmeshChoice) 3)
    (Variables|Default|SetmeshChoice 0)
    (else
      (Math|Integer|IncrementInt (Variables|Default|GetmeshChoice)
        (:%20%20
          _))))
  (CallFunction|SetMesh (Variables|Default|GetCharacterMeshArray) (Variables|Default|GetmeshChoice)))

(event EventBeginPlay
  ;[1 1 1] create character mesh array and set based on character choice
  (CallFunction|SpawnSaber)
  (CallFunction|StartFunction))

(event EventTick
  (params (DeltaSeconds :type Float%20%28single-precision%29))
  (CallFunction|Movement DeltaSeconds)
  (CallFunction|GrappleDespawnCollision)
  (CallFunction|CollisionCheck)
  (Transformation|SetActorRotation "0, 0, 0")
  (CallFunction|GrapplingFunction)
  (CallFunction|RotateGrappleArrow (Input|AxisValues|GetMoveRight) (Input|AxisValues|GetMoveUp))
  (CallFunction|WallClimbing)
  (if (Variables|Grapple|GetIsGrappling)
    (Class|PhysicsCharacterSC|RopeCollision (Variables|Default|GetPhysicsCharacterSC))
    (CallFunction|RopeChanges))
  (CallFunction|RotateSaber (Input|AxisValues|GetSaberRight) (Input|AxisValues|GetSaberUp))
  (CallFunction|UpdateLives)
  (CallFunction|RotateMesh)
  (Variables|Player|SetCurrentVelocity (Transformation|GetVelocity))
  (if (Variables|WallClimbing|GetAddedEdgeForce)
    (Utilities|FlowControl|Delay 1.0)
    (Variables|WallClimbing|SetAddedEdgeForce false)
    (else
      (CallFunction|ClimbLedge))))

(event Input|ActionEvents|InputActionJump
  (params (Key :type Key%20Structure :default "None"))
  (:Pressed
    (CallFunction|Jump)
    (Utilities|FlowControl|Delay 0.5)
    (Variables|WallClimbing|SetWallJumping false)
    (Utilities|FlowControl|Delay 0.1 :!label _label)
    (if (Variables|Collision|GetOnGround)
      (Variables|Movement|SetJumping false)
      (else
        (goto _label)))))

(event Input|ActionEvents|InputActionGrapple
  (params (Key :type Key%20Structure :default "None"))
  (:Pressed
    (if (Variables|Grapple|GetGrappleCooldown)
      (CallFunction|GrapplePress)
      (Utilities|FlowControl|Delay 0.5)
      (Variables|Grapple|SetFloorWallGrapple true)
      (Variables|Grapple|SetGrappleFromWall false)
      (Variables|Grapple|SetGrappleCooldown false)
      (Utilities|FlowControl|Delay (Variables|Grapple|GetGrappleCooldownLength))
      (Variables|Grapple|SetGrappleCooldown true)))
  (:Released
    (CallFunction|DespawnGrapple)))

(event Input|ActionEvents|InputActionLungeAttack
  (params (Key :type Key%20Structure :default "None"))
  (:Pressed
    (CallFunction|ChargeAttack :!label _label)
    (Utilities|FlowControl|Delay 0.5)
    (if (Variables|ChargeAttack|GetCharging)
      (goto _label)))
  (:Released
    (CallFunction|LungeAttack)))

(event Input|ActionEvents|InputActionChangeCharacterLeft
  (params (Key :type Key%20Structure :default "None"))
  (:Pressed
    (CallFunction|CycleLeftMesh)))

(event Input|ActionEvents|InputActionChangeCharacterRight
  (params (Key :type Key%20Structure :default "None"))
  (:Pressed
    (CallFunction|CycleRightMesh)))

(event Input|ActionEvents|InputActionChangeMaterialLeft
  (params (Key :type Key%20Structure :default "None"))
  ;[1 1 1] cycling through different colours
  (:Pressed
    (if (<= (Variables|Default|GetmaterialChoice) 0)
      (Variables|Default|SetmaterialChoice 3)
      (else
        (Math|Integer|DecrementInt (Variables|Default|GetmaterialChoice)
          (:%20%20
            _))))
    (CallFunction|SetMaterial (Variables|Default|GetMaterialMC_Array) (Variables|Default|GetmaterialChoice))))

(event Input|ActionEvents|InputActionChangeMaterialRight
  (params (Key :type Key%20Structure :default "None"))
  ;[1 1 1] cycling through different colours
  (:Pressed
    (if (>= (Variables|Default|GetmaterialChoice) 3)
      (Variables|Default|SetmaterialChoice 0)
      (else
        (Math|Integer|DecrementInt (Variables|Default|GetmaterialChoice)
          (:%20%20
            _))))
    (CallFunction|SetMaterial (Variables|Default|GetMaterialMC_Array) (Variables|Default|GetmaterialChoice))))

(event Input|ActionEvents|InputActionStart
  (params (Key :type Key%20Structure :default "None")))

(event Input|AxisEvents|InputAxisMoveRight
  (params (AxisValue :type Float%20%28single-precision%29))
  (Variables|Movement|SetMoveDirection (Math|Vector|MakeVector 0.0 (Math|Float|Clamp(Float) AxisValue -1.0) 0.0)))

(fn ConstructionScript
  (CallFunction|SetMesh (Variables|Default|GetCharacterMeshArray) (Variables|Default|GetmeshChoice))
  (CallFunction|SetMaterial (Variables|Default|GetMaterialMC_Array) (Variables|Default|GetmaterialChoice)))

(fn Movement
  (params (DeltaTime :type Float%20%28single-precision%29))
  (bind _movedirection (Variables|Movement|GetMoveDirection))
  (if (not (Math|Vector|VectorIsZero _movedirection))
    (if (or (Variables|Collision|GetLeftCollision) (Variables|Collision|GetRightCollision))
      (if (or (and (> (.y (Variables|Movement|GetMoveDirection)) 0.0) (Variables|Collision|GetLeftCollision)) (and (< (.y (Variables|Movement|GetMoveDirection)) -0.1) (Variables|Collision|GetRightCollision)))
        (if (and (Variables|WallClimbing|GetIsClimbing) (Variables|WallClimbing|GetCanWallClimb)) :!label _label
          (if (Variables|WallClimbing|GetWallJumping)
            (if (Variables|Collision|GetOnGround) :!label _label_2
              (Transformation|SetActorLocation (+ (Transformation|GetActorLocation) (* (* _movedirection DeltaTime) (Variables|Movement|GetMovementSpeed))) false false :!label _label_3)
              (elif (Variables|Movement|GetJumping)
                (Physics|AddForce (Variables|Default|GetBox) (Math|Vector|MakeVector 0.0 (* (.y (Variables|Movement|GetMoveDirection)) (* (Variables|Movement|GetMidAirMoveSpeed) -1.0)) 0.0) "None" true)
                (else
                  (goto _label_3)))))
          (else
            (goto _label_2))))
      (else
        (goto _label)))))

(fn CollisionCheck
  (bind _returnvalue (Transformation|GetActorLocation))
  (bind _returnvalue_2 (Transformation|GetActorLocation))
  (bind _returnvalue_3 (Transformation|GetActorLocation))
  (bind _returnvalue_4 (Transformation|GetActorLocation))
  (bind _returnvalue_5 (Transformation|GetActorLocation))
  (bind _returnvalue_6 (Transformation|GetActorLocation))
  (bind _box (Variables|Default|GetBox))
  (bind _box_2 (Variables|Default|GetBox))
  (bind _returnvalue_7 (Math|Vector|GetRightVector _box))
  (bind _returnvalue_8 (Math|Vector|GetRightVector _box_2))
  (bind _returnvalue_9 (* _returnvalue_7 75.0))
  (bind _returnvalue_10 (* _returnvalue_8 -75.0))
  (bind _returnvalue_11 (+ (Math|Vector|MakeVector (.x _returnvalue) (.y _returnvalue) (.z _returnvalue)) _returnvalue_9))
  (bind _returnvalue_12 (+ (Math|Vector|MakeVector (.x _returnvalue_4) (.y _returnvalue_4) (.z _returnvalue_4)) _returnvalue_10))
  (bind (_outhit _returnvalue_13) (Collision|LineTraceByChannel _returnvalue_2 (+ _returnvalue_2 (* (Math|Vector|GetRightVector (Variables|Default|GetBox)) -75.0)) "TraceTypeQuery1" false 0 "ForDuration" true "(R=1.000000,G=0.000000,B=0.000000,A=1.000000)" "(R=0.000000,G=1.000000,B=0.000000,A=1.000000)" 0.1))
  (bind _output_get (Variables|Collision|SetRightCollision _returnvalue_13))
  (if _output_get
    (Variables|WallClimbing|SetCanWallClimb (Components|ComponentHasTag (.HitComponent (Collision|BreakHitResult _outhit)) "Wall")))
  (bind (_outhit_2 _returnvalue_14) (Collision|LineTraceByChannel _returnvalue_3 (+ _returnvalue_3 (* (Math|Vector|GetRightVector (Variables|Default|GetBox)) 75.0)) "TraceTypeQuery1" false 0 "ForDuration" true "(R=1.000000,G=0.000000,B=0.000000,A=1.000000)" "(R=0.000000,G=1.000000,B=0.000000,A=1.000000)" 0.1))
  (bind _output_get_2 (Variables|Collision|SetLeftCollision _returnvalue_14))
  (if _output_get_2
    (Variables|WallClimbing|SetCanWallClimb (Components|ComponentHasTag (.HitComponent (Collision|BreakHitResult _outhit_2)) "Wall")))
  (if (and (Math|Boolean|Equal(Boolean) (Variables|Collision|GetLeftCollision) false) (Math|Boolean|Equal(Boolean) (Variables|Collision|GetRightCollision) false))
    (Variables|WallClimbing|SetCanWallClimb false))
  (bind _returnvalue_15 (Collision|LineTraceByChannel _returnvalue_5 (+ _returnvalue_5 (* (Math|Vector|GetUpVector (Variables|Default|GetBox)) -1e+02)) "TraceTypeQuery1" false 0 "ForDuration" true "(R=1.000000,G=0.000000,B=0.000000,A=1.000000)" "(R=0.000000,G=1.000000,B=0.000000,A=1.000000)" 0.1))
  (Variables|Collision|SetOnGround _returnvalue_15)
  (bind _returnvalue_16 (Collision|LineTraceByChannel _returnvalue_6 (+ _returnvalue_6 (* (Math|Vector|GetUpVector (Variables|Default|GetBox)) 75.0)) "TraceTypeQuery1" false 0 "None" true "(R=1.000000,G=0.000000,B=0.000000,A=1.000000)" "(R=0.000000,G=1.000000,B=0.000000,A=1.000000)" 0.1))
  (Variables|Collision|SetUpCollision _returnvalue_16)
  (bind (_outhit_3 _returnvalue_17) (Collision|LineTraceByChannel (Math|Vector|MakeVector (.x _returnvalue_4) (.y _returnvalue_4) (- (.z _returnvalue_4) 1e+01)) (Math|Vector|MakeVector (.x _returnvalue_12) (.y _returnvalue_12) (- (.z _returnvalue_12) 1e+01)) "TraceTypeQuery1" false 0 "ForDuration" true "(R=1.000000,G=0.000000,B=0.000000,A=1.000000)" "(R=0.000000,G=1.000000,B=0.000000,A=1.000000)" 0.1))
  (if _returnvalue_17
    (Variables|Collision|SetTopClimbRight (Components|ComponentHasTag (.HitComponent (Collision|BreakHitResult _outhit_3)) "Wall"))
    (else
      (Variables|Collision|SetTopClimbRight false)))
  (bind (_outhit_4 _returnvalue_18) (Collision|LineTraceByChannel (Math|Vector|MakeVector (.x _returnvalue) (.y _returnvalue) (- (.z _returnvalue) 1e+01)) (Math|Vector|MakeVector (.x _returnvalue_11) (.y _returnvalue_11) (- (.z _returnvalue_11) 1e+01)) "TraceTypeQuery1" false 0 "ForDuration" true "(R=1.000000,G=0.000000,B=0.000000,A=1.000000)" "(R=0.000000,G=1.000000,B=0.000000,A=1.000000)" 0.1))
  (if _returnvalue_18
    (Variables|Collision|SetTopClimbLeft (Components|ComponentHasTag (.HitComponent (Collision|BreakHitResult _outhit_4)) "Wall"))
    (else
      (Variables|Collision|SetTopClimbLeft false))))

(fn Jump
  (bind _walljumpheight (Variables|Movement|GetWallJumpHeight))
  (bind _box (Variables|Default|GetBox))
  (bind _grapplearrow (Variables|Default|GetGrappleArrow))
  (bind _returnvalue (Math|Vector|GetForwardVector _grapplearrow))
  (if (Variables|Collision|GetOnGround)
    (Variables|Movement|SetJumping true)
    (Physics|AddImpulse (Variables|Default|GetBox) (Math|Vector|MakeVector 0.0 (* (.y (Variables|Movement|GetMoveDirection)) (* (Variables|Movement|GetMidAirMoveSpeed) -1.0)) (Variables|Movement|GetJumpHeight)) "None" true))
  (if (and (Variables|WallClimbing|GetCanWallClimb) (Variables|WallClimbing|GetIsClimbing))
    (Physics|SetEnableGravity _box true)
    (Physics|AddImpulse _box (Math|Vector|MakeVector 0.0 (* (.y _returnvalue) _walljumpheight) (* (.z _returnvalue) _walljumpheight)) "None" true)
    (Variables|WallClimbing|SetWallJumping true)
    (Variables|Movement|SetJumping true)))

(fn GrapplePress
  (bind _physicscharactersc (Variables|Default|GetPhysicsCharacterSC))
  (bind _c1 (Variables|Default|GetC1))
  (Class|PhysicsCharacterSC|RaycastPhysicsChar _physicscharactersc (Variables|Default|GetGrappleArrow) (Variables|Grapple|GetGrappleRange))
  (if (Variables|/Script/QuantumCollapse.PhysicsCharacterSC|GethasHitGrapple _physicscharactersc)
    (Variables|Grapple|SetIsGrappling true)
    (Variables|/Script/CableComponent.CableComponent|SetbEnableCollision _c1 true)
    (Rendering|SetVisibility _c1 true false)
    (bind _returnvalue (Game|SpawnActorfromClass "/Game/Actors/Sphere.Sphere_C" (Math|Transform|MakeTransform (Variables|/Script/QuantumCollapse.PhysicsCharacterSC|GetgrappleAnchorPoint (Variables|Default|GetPhysicsCharacterSC)) "0, 0, 0" "1,1,1") "Undefined" 0 0 0))
    (Class|CableComponent|SetAttachEndto (Variables|Default|GetC1) _returnvalue "None" "None")
    (Variables|Grapple|SetGrappleHookObj _returnvalue)
    (Rendering|SetVisibility (Variables|/Script/Engine.Actor|GetRootComponent (Variables|Grapple|GetGrappleHookObj)) false false)
    (Variables|Grapple|SetGrappleFromWall true)))

(fn DespawnGrapple
  (bind _c1 (Variables|Default|GetC1))
  (Variables|Grapple|SetIsGrappling false)
  (Variables|Grapple|SetFloorWallGrapple false)
  (Rendering|SetVisibility _c1 false false)
  (Variables|/Script/CableComponent.CableComponent|SetbEnableCollision _c1 false))

(fn GrapplingFunction
  (if (Variables|Grapple|GetIsGrappling)
    (bind _returnvalue (Class|PhysicsCharacterSC|CalculateGrappleForcePhysicsChar (Variables|Default|GetPhysicsCharacterSC) (Input|AxisValues|GetMoveRight) (Variables|Grapple|GetGrappleForce)))
    (Physics|AddImpulse (Variables|Default|GetBox) _returnvalue "None" true)))

(fn RotateGrappleArrow
  (params (xValue :type Float%20%28single-precision%29) (yValue :type Float%20%28single-precision%29))
  (if (or (!= xValue 0.0) (!= yValue 0.0))
    (Variables|Grapple|SetGrappleArrowDirection (Class|KismetMathLibrary|DegAtan2 yValue xValue))
    (Transformation|SetWorldRotation (Variables|Default|GetGrappleArrow) (Math|Rotator|MakeRotator 0.0 (Variables|Grapple|GetGrappleArrowDirection) -9e+01) false false)))

(fn WallClimbing
  (bind _returnvalue (Transformation|GetActorLocation))
  (bind _returnvalue_2 (Input|AxisValues|GetMoveUp))
  (bind _box (Variables|Default|GetBox))
  (if (not (Variables|Grapple|GetGrappleFromWall))
    (if (not (Variables|WallClimbing|GetWallJumping))
      (Variables|WallClimbing|SetIsClimbing (or (Variables|Collision|GetLeftCollision) (Variables|Collision|GetRightCollision)))
      (if (and (<= (Input|AxisValues|GetMoveUp) 0.0) (Variables|Collision|GetOnGround))
        (Variables|WallClimbing|SetIsClimbing false))
      (if (and (Variables|WallClimbing|GetIsClimbing) (Variables|WallClimbing|GetCanWallClimb))
        (if (Variables|Collision|GetUpCollision)
          (if (< _returnvalue_2 0.0)
            (Variables|Movement|SetMoveDirection (Math|Vector|MakeVector 0.0 0.0 (Math|Float|Clamp(Float) (Input|AxisValues|GetMoveUp) -1.0)) :!label _label)
            (Physics|SetEnableGravity _box false)
            (Physics|SetPhysicsLinearVelocity _box "0, 0, 0" false "None")
            (Transformation|SetActorLocation (Math|Vector|MakeVector (.x _returnvalue) (.y _returnvalue) (+ (* (Input|AxisValues|GetMoveUp) (Variables|WallClimbing|GetClimbingSpeed)) (.z _returnvalue))) false false))
          (elif (Variables|Collision|GetOnGround)
            (if (> _returnvalue_2 0.1)
              (goto _label)
              (else
                (Physics|SetEnableGravity (Variables|Default|GetBox) true :!label _label_2)))
            (else
              (goto _label))))
        (else
          (goto _label_2))))))

(fn SpawnSaber
  (bind _returnvalue (Game|SpawnActorfromClass "/Game/Prototype/BenTesting/LightSaber/SaberBP.SaberBP_C" (Transformation|GetSocketTransform (Variables|Default|GetSkeletalMesh) "SaberSocket" "RTS_World") "Undefined" 0 0 0))
  (Variables|Saber|SetSaber _returnvalue)
  (Transformation|AttachComponentToComponent _returnvalue (Variables|Default|GetSkeletalMesh) "SaberSocket" "SnapToTarget" "SnapToTarget" "SnapToTarget" true))

(fn RotateSaber
  (params (X%20Value :type Float%20%28single-precision%29) (Y%20Value :type Float%20%28single-precision%29))
  (Transformation|SetActorLocation (Variables|Saber|GetSaber) (Transformation|GetActorLocation) false false)
  (if (or (!= X%20Value 0.0) (!= Y%20Value 0.0))
    (Variables|Saber|SetSaberDirection (Class|KismetMathLibrary|DegAtan2 (* Y%20Value -1.0) X%20Value)))
  (Transformation|SetActorLocation (Variables|Saber|GetSaber) (Transformation|GetSocketLocation (Variables|Default|GetSkeletalMesh) "SaberSocket") false false))

(fn UpdateLives
  (Variables|Player|SetLives (Variables|/Script/QuantumCollapse.PhysicsCharacterSC|Getlives (Variables|Default|GetPhysicsCharacterSC))))

(fn StartFunction
  (Variables|/Script/QuantumCollapse.PhysicsCharacterSC|Setlives (Variables|Default|GetPhysicsCharacterSC) (Variables|Player|GetLives))
  (Game|SpawnActorfromClass "/Game/Actors/Sphere.Sphere_C" (Math|Transform|MakeTransform "0, 0, 0" "0, 0, 0" "1,1,1") "Undefined" 0 0 0)
  (bind _outactors (Actor|GetAllActorsOfClass "/Game/GameManagerBP.GameManagerBP_C"))
  (Variables|Player|SetGame%20Manager (Utilities|Array|Get(acopy) _outactors)))

(fn RopeChanges
  (bind _grapplehookobj (Variables|Grapple|GetGrappleHookObj))
  (Variables|/Script/CableComponent.CableComponent|SetCableLength (Variables|Default|GetC1) (Math|Vector|Distance(Vector) (Transformation|GetActorLocation) (Variables|/Script/QuantumCollapse.PhysicsCharacterSC|GetgrappleAnchorPoint (Variables|Default|GetPhysicsCharacterSC))))
  (if (!= _grapplehookobj 0)
    (Transformation|SetActorLocation _grapplehookobj (Variables|/Script/QuantumCollapse.PhysicsCharacterSC|GetraycastHitPoint (Variables|Default|GetPhysicsCharacterSC)) false false)))

(fn GrappleDespawnCollision
  (if (and (Math|Boolean|ORBoolean (Variables|Collision|GetLeftCollision) (Variables|Collision|GetRightCollision) (Variables|Collision|GetOnGround) (Variables|Collision|GetUpCollision)) (Variables|Grapple|GetFloorWallGrapple))
    (CallFunction|DespawnGrapple)))

(fn LungeAttack
  (Variables|ChargeAttack|SetCharging false)
  (Physics|AddImpulse (Variables|Default|GetBox) (* (* (Math|Vector|GetForwardVector (Variables|/Game/Prototype/BenTesting/LightSaber/SaberBP.SaberBP_C|GetDefaultSceneRoot (Variables|Saber|GetSaber))) (* (Variables|ChargeAttack|GetChargeTime) (Variables|ChargeAttack|GetChargeVelocity))) -1.0) "None" true)
  (Variables|ChargeAttack|SetChargeTime 0.0))

(fn ChargeAttack
  (bind _output_get (Variables|ChargeAttack|SetCharging true))
  (if _output_get
    (Variables|ChargeAttack|SetChargeTime (Math|Float|Clamp(Float) (+ (Variables|ChargeAttack|GetChargeTime) (Variables|ChargeAttack|GetChargeTimeTicRate)) 0.0 (Variables|ChargeAttack|GetMaxChargeAttack)))
    (Development|PrintString "pressed")))

(fn ClimbLedge
  (if (Variables|Collision|GetTopClimbRight)
    (if (not (Variables|WallClimbing|GetIsClimbing))
      (if (not (Variables|WallClimbing|GetAddedEdgeForce))
        (Physics|AddImpulse (Variables|Default|GetBox) "0,-10.000000,750.000000" "None" true)
        (Variables|WallClimbing|SetAddedEdgeForce true)))
    (elif (Variables|Collision|GetTopClimbLeft)
      (if (not (Variables|WallClimbing|GetIsClimbing))
        (if (not (Variables|WallClimbing|GetAddedEdgeForce))
          (Physics|AddImpulse (Variables|Default|GetBox) "0,10.000000,750.000000" "None" true)
          (Variables|WallClimbing|SetAddedEdgeForce true))))))

(fn RotateMesh
  (bind _skeletalmesh (Variables|Default|GetSkeletalMesh))
  (if (or (> (Variables|Saber|GetSaberDirection) 9e+01) (< (Variables|Saber|GetSaberDirection) -9e+01))
    (Transformation|SetRelativeRotation _skeletalmesh "0, 0, 0" false false)
    (Variables|Animations|SetMeshRotated true)
    (else
      (Transformation|SetRelativeRotation _skeletalmesh "0,-180.000000, 0" false false)
      (Variables|Animations|SetMeshRotated false))))

(fn AssignColourOutline
  (if (== (Class|GameplayStatics|GetPlayerControllerID (Class|GameplayStatics|GetPlayerControllerfromID)) 0)
    (Variables|Outline|SetPlayer%20Outline%20Number 1)
    (Rendering|SetCustomDepthStencilValue (Variables|Default|GetSkeletalMesh) (Variables|Outline|GetPlayer%20Outline%20Number) :!label _label)
    (elif (== (Class|GameplayStatics|GetPlayerControllerID (Class|GameplayStatics|GetPlayerControllerfromID 1)) 1)
      (Variables|Outline|SetPlayer%20Outline%20Number 2)
      (goto _label)
      (elif (== (Class|GameplayStatics|GetPlayerControllerID (Class|GameplayStatics|GetPlayerControllerfromID 2)) 2)
        (Variables|Outline|SetPlayer%20Outline%20Number 3)
        (goto _label)
        (elif (== (Class|GameplayStatics|GetPlayerControllerID (Class|GameplayStatics|GetPlayerControllerfromID 3)) 3)
          (Variables|Outline|SetPlayer%20Outline%20Number 4)
          (goto _label))))))

(fn SetMaterial
  (params (Material%20Array%20To%20Use :type Array%20of%20Material%20Instance%20Object%20References) (Material%20Choice :type Integer))
  (Rendering|Material|SetMaterial (Variables|Default|GetSkeletalMesh) 0 (Utilities|Array|Get(acopy) Material%20Array%20To%20Use Material%20Choice)))

(fn SetMesh
  (params (Mesh%20Array%20to%20use :type Array%20of%20Skeletal%20Mesh%20Object%20References) (Mesh%20Choice :type Integer))
  (Class|SkinnedMeshComponent|SetSkeletalMesh (Variables|Default|GetSkeletalMesh) (Utilities|Array|Get(acopy) Mesh%20Array%20to%20use Mesh%20Choice) true))
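; SpawnPlayerInstances activates the first player's character in the scene based on player count data held in the game instance.
; Its SpawnInScene event casts the game instance to NewGameInstance and prints PlayerCount1 for debugging.
; When that value converts to true, it unhides player character 0 and enables its collision, revealing an existing character rather than spawning a new one.
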(event Custom|SpawnInScene
  (bind _asnew_game_instance (Utilities|Casting|CastToNewGameInstance (Game|GetGameInstance)))
  (Development|PrintString (Utilities|String|ToString(Integer) (Variables|/Game/SideScrollerCPP/Blueprints/NewGameInstance.NewGameInstance_C|GetPlayerCount1 _asnew_game_instance)))
  (if (Math|Conversions|ToBoolean(Integer) (Variables|/Game/SideScrollerCPP/Blueprints/NewGameInstance.NewGameInstance_C|GetPlayerCount1 _asnew_game_instance))
    (Rendering|SetActorHiddenInGame (Game|GetPlayerCharacter 0) false)
    (Collision|SetActorEnableCollision (Game|GetPlayerCharacter 0) true)))
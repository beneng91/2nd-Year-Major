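; Prototype character-cycling Blueprint that spawns characters at random PlayerStarts and lets the player switch possession between them.
; The Start input loops up to the selected index and, on a failed validity check, refreshes the PlayerStart array, spawns a character and adds it to PlayerCharacters.
; Both ChangeCharacter inputs share one path that prints the index, advances it with wraparound and possesses that character, so left and right cycle in the same direction.
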(event EventBeginPlay)

(event EventTick
  (params (DeltaSeconds :type Float%20%28single-precision%29)))

(event Input|ActionEvents|InputActionStart
  (params (Key :type Key%20Structure))
  (:Pressed
    (for _index (range 0 (Variables|Default|GetCurrentlySelectedCharacterIndex))
      (Utilities|IsValid 0
        (:Is%20Not%20Valid
          (CallFunction|PlayerStartLocation)
          (bind _player_start_location (CallFunction|GetStartLocation))
          (bind _returnvalue (Game|SpawnActorfromClass "/Game/SideScrollerCPP/Blueprints/NewCharacter.NewCharacter_C" (Math|Conversions|ToTransform(Vector) _player_start_location) "Undefined" 0 2.5e+03 5e+02 5e+01 "0.000000,0.000000,0.000000" 5e+03 0 3 0))
          (Utilities|Array|Add (Variables|Default|GetPlayerCharacters) _returnvalue))))))

(event Input|ActionEvents|InputActionChangeCharacterLeft
  (params (Key :type Key%20Structure))
  (:Pressed
    (Development|PrintString (Utilities|String|ToString(Integer) (Variables|Default|GetCurrentlySelectedCharacterIndex)))
    (Variables|Default|SetCurrentlySelectedCharacterIndex (Math|Integer|%(Integer) (+ (Variables|Default|GetCurrentlySelectedCharacterIndex) 1) (Utilities|Array|Length (Variables|Default|GetPlayerCharacters))))
    (Pawn|Possess (Game|GetPlayerController (Variables|Default|GetAllPlayers)) (Utilities|Array|Get(acopy) (Variables|Default|GetPlayerCharacters) (Variables|Default|GetCurrentlySelectedCharacterIndex)))))

(event Input|ActionEvents|InputActionChangeCharacterRight
  (params (Key :type Key%20Structure))
  (:Pressed
    (Development|PrintString (Utilities|String|ToString(Integer) (Variables|Default|GetCurrentlySelectedCharacterIndex)))
    (Variables|Default|SetCurrentlySelectedCharacterIndex (Math|Integer|%(Integer) (+ (Variables|Default|GetCurrentlySelectedCharacterIndex) 1) (Utilities|Array|Length (Variables|Default|GetPlayerCharacters))))
    (Pawn|Possess (Game|GetPlayerController (Variables|Default|GetAllPlayers)) (Utilities|Array|Get(acopy) (Variables|Default|GetPlayerCharacters) (Variables|Default|GetCurrentlySelectedCharacterIndex)))))

(fn ConstructionScript)

(fn PlayerStartLocation
  (bind _outactors (Actor|GetAllActorsOfClass "/Script/Engine.PlayerStart"))
  (Variables|Default|SetPlayerStartArray _outactors))

(fn GetStartLocation
  (return (Transformation|GetActorLocation (Utilities|Array|Get(acopy) (Variables|Default|Getplayerstartarray) (Math|Random|RandomIntegerinRange 0 (- (Utilities|Array|Length (Variables|Default|Getplayerstartarray)) 1))))))
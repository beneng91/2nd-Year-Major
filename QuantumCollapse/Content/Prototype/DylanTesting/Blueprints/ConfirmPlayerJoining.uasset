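; ConfirmPlayerJoining carries character select choices into the next level through the game instance.
; Its playertransition event loops over the Csplayer array, writing each skeletal mesh and first material into game instance arrays by index and incrementing PlayerNumbers.
; It then opens the level named by LevelName.
; An alternative append-based copy sits on a branch that never runs, as its condition is fixed to true.
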(event Custom|playertransition
  (bind _gameinstance (Variables|Default|Getgameinstance))
  (bind _gameinstance_2 (Variables|Default|Getgameinstance))
  (if true
    (for (_array_element _array_index) (Variables|Default|Getcsplayer)
      (Utilities|Array|SetArrayElem (Variables|/Game/SideScrollerCPP/Blueprints/NewGameInstance.NewGameInstance_C|GetCharacterSelectMeshes _gameinstance) _array_index (Variables|/Script/Engine.SkinnedMeshComponent|GetSkeletalMesh (Variables|/Game/Prototype/Liam/CS_Player.CS_Player_C|GetSkeletalMesh _array_element)))
      (Utilities|Array|SetArrayElem (Variables|/Game/SideScrollerCPP/Blueprints/NewGameInstance.NewGameInstance_C|GetCharacterSelectMaterials1 _gameinstance) _array_index (Rendering|Material|GetMaterial (Variables|/Game/Prototype/Liam/CS_Player.CS_Player_C|GetSkeletalMesh _array_element) 0))
      (Variables|/Game/SideScrollerCPP/Blueprints/NewGameInstance.NewGameInstance_C|SetPlayerNumbers _gameinstance (+ (Variables|/Game/SideScrollerCPP/Blueprints/NewGameInstance.NewGameInstance_C|GetPlayerNumbers _gameinstance) 1)))
    (else
      (for _array_element_2 (Variables|Default|Getcsplayer)
        (if true
          (Utilities|Array|Add (Variables|/Game/SideScrollerCPP/Blueprints/NewGameInstance.NewGameInstance_C|GetCharacterSelectMeshes _gameinstance_2) (Variables|/Script/Engine.SkinnedMeshComponent|GetSkeletalMesh (Variables|/Game/Prototype/Liam/CS_Player.CS_Player_C|GetSkeletalMesh _array_element_2)))
          (Utilities|Array|Add (Variables|/Game/SideScrollerCPP/Blueprints/NewGameInstance.NewGameInstance_C|GetCharacterSelectMaterials1 _gameinstance_2) (Rendering|Material|GetMaterial (Variables|/Game/Prototype/Liam/CS_Player.CS_Player_C|GetSkeletalMesh _array_element_2) 0))
          (Variables|/Game/SideScrollerCPP/Blueprints/NewGameInstance.NewGameInstance_C|SetPlayerNumbers _gameinstance_2 (+ (Variables|/Game/SideScrollerCPP/Blueprints/NewGameInstance.NewGameInstance_C|GetPlayerNumbers _gameinstance_2) 1))))))
  (Game|OpenLevel(byName) (Variables|Default|GetLevel%20Name)))

(fn ConstructionScript)
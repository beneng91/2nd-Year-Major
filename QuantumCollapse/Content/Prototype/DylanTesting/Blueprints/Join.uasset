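; Prototype join Blueprint that populates the match with CS_Player characters when play begins.
; PlayersConnect spawns one character at every PlayerStart and adds it to the CS_GameStateBase player list.
; The loop index sets each character's player number, outline, mesh and material, with the skin applied through WinningPlayerChanges.
; No controller possession or input assignment happens here, and a failed game state cast only prints an error.
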(event EventBeginPlay
  (CallFunction|PlayersConnect))

(fn ConstructionScript)

(fn PlayersConnect
  (bind _ascs_game_state_base (Utilities|Casting|CastToCS_GameStateBase (Game|GetGameState))
    (:then
      (bind _outactors (Actor|GetAllActorsOfClass "/Script/Engine.PlayerStart"))
      (bind _output_get (Variables|Default|Setplayerstartarray _outactors))
      (for (_array_element _array_index) _output_get
        (bind _returnvalue (Game|SpawnActorfromClass "/Game/Prototype/Liam/CS_Player.CS_Player_C" (Transformation|GetActorTransform _array_element) "AlwaysSpawn" 0 (+ _array_index 1) 0))
        (Utilities|Array|AddUnique (Variables|/Game/Blueprints/CS_GameStateBase.CS_GameStateBase_C|GetCS_PlayerList _ascs_game_state_base) _returnvalue)
        (Variables|/Game/Prototype/Liam/CS_Player.CS_Player_C|SetPlayerNumber _returnvalue (+ _array_index 1))
        (Variables|/Game/Prototype/Liam/CS_Player.CS_Player_C|SetMeshInstance _returnvalue _array_index)
        (Variables|/Game/Prototype/Liam/CS_Player.CS_Player_C|SetMaterialInstance _returnvalue _array_index)
        (Default|WinningPlayerChanges _returnvalue (Utilities|Array|Get(acopy) (Variables|/Game/Prototype/Liam/CS_Player.CS_Player_C|GetCharacterSkinArray _returnvalue) _array_index) (Utilities|Array|Get(acopy) (Variables|/Game/Prototype/Liam/CS_Player.CS_Player_C|GetMaterialInstancesArray _returnvalue) _array_index))))
    (:CastFailed
      (Development|PrintString "Base Game State Broken" true true "(R=1.000000,G=0.000000,B=0.033375,A=1.000000)" 1e+03))))
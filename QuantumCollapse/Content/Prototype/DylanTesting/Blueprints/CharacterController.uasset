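; Prototype player controller that lets the player pick a character and swaps the controlled pawn to match.
; On BeginPlay it stores the starting pawn and shows a selection widget in UI-only input mode with the mouse cursor visible.
; CharacterSelection looks up the choice in a class map, spawns that class at the current pawn's transform and possesses it.
; It then restores game-only input, removes the widget and destroys the original pawn.
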(event EventCharacterSelection
  (params (Selection :type Integer))
  (bind _charactermap (Variables|Default|GetCharacterMap))
  (bind (_value _returnvalue) (Utilities|Map|Find _charactermap Selection))
  (if _returnvalue
    (Development|PrintString (Utilities|GetClassDisplayName _value))
    (bind _returnvalue_2 (Game|SpawnActorfromClass _value (Transformation|GetActorTransform (Pawn|GetControlledPawn)) "Undefined" 0 2.5e+03 5e+02 5e+01 "0.000000,0.000000,0.000000" 5e+03 0 3 0))
    (bind _output_get (Variables|Default|SetPossessPawn _returnvalue_2))
    (Pawn|Possess self _output_get)
    (Input|SetInputModeGameOnly self)
    (Widget|RemovefromParent (Variables|Default|GetSelectCharacterRef))
    (Actor|DestroyActor (Variables|Default|GetOld%20Pawn))))

(event EventBeginPlay
  (Variables|Default|SetOld%20Pawn (Pawn|GetControlledPawn))
  (bind _returnvalue (UserInterface|CreateWidget "/Game/Prototype/DylanTesting/Menus/WidgetBlueprints/CharacterSelect.CharacterSelect_C" self))
  (Variables|Default|SetSelectCharacterRef _returnvalue)
  (UserInterface|Viewport|AddtoViewport (Variables|Default|GetSelectCharacterRef) 0)
  (Variables|Default|SetbShowMouseCursor self true)
  (Input|SetInputModeUIOnly self (Variables|/Game/Prototype/DylanTesting/Menus/WidgetBlueprints/CharacterSelect.CharacterSelect_C|GetPlayer1 (Variables|Default|GetSelectCharacterRef)) "DoNotLock"))

(fn ConstructionScript)
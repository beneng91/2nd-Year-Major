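; MainMode is a prototype local multiplayer setup Blueprint that creates players from the level's PlayerStarts.
; After a short delay on BeginPlay, it gathers them and creates a player for each array index matching a numeric PlayerStartTag.
; Each gets a possessed BP_InputReciever, placed by array index rather than the tag-matched start.
; SpawnCharacter, uncalled here, responds once to a gamepad key by calling the GameMode's SpawnCharacters with controller 1's ID.
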(event EventBeginPlay
  (Utilities|FlowControl|Delay 0.2)
  (CallFunction|PlayerStart)
  (CallFunction|InputReciever))

(event EventTick
  (params (DeltaSeconds :type Float%20%28single-precision%29)))

(fn ConstructionScript)

(fn PlayerStart
  (bind _outactors (Actor|GetAllActorsOfClass "/Script/Engine.PlayerStart"))
  (Variables|Default|SetPlayerStartArray _outactors))

(fn InputReciever
  (for (_ _array_index) (Variables|Default|GetPlayerStartArray)
    (LocalVariables|SetIndex _array_index)
    (for _array_element (Variables|Default|GetPlayerStartArray)
      (if (== (CallFunction|NametoInt _array_element) (LocalVariables|GetIndex))
        (Class|GameplayStatics|CreatePlayer (LocalVariables|GetIndex))
        (bind _returnvalue (Game|SpawnActorfromClass "/Game/SideScrollerCPP/Blueprints/BP_InputReciever.BP_InputReciever_C" (Transformation|GetActorTransform (Utilities|Array|Get(acopy) (Variables|Default|GetPlayerStartArray) (LocalVariables|GetIndex))) "Undefined" 0 (LocalVariables|GetIndex) 0 0 0))
        (Utilities|Array|AddUnique (Variables|Default|GetPlayerInputRecieverArray) _returnvalue)
        (Pawn|Possess (Game|GetPlayerController (LocalVariables|GetIndex)) _returnvalue)
        (Utilities|Array|AddUnique (Variables|Default|GetPlayerControllerArray) (Game|GetPlayerController (LocalVariables|GetIndex)))))))

(fn NametoInt
  (params (PlayerStart :type Player%20Start%20Object%20Reference))
  (return (Math|Conversions|ToInteger(Byte) (Utilities|String|ToString(Name) (Variables|/Script/Engine.PlayerStart|GetPlayerStartTag PlayerStart)))))

(fn SpawnCharacter
  (params (Key :type Key%20Structure%20%28by%20ref%29))
  (if (Class|KismetInputLibrary|KeyIsGamepadKey Key)
    (Utilities|FlowControl|DoOnce false
      (:Completed
        (bind _asgame_mode (Utilities|Casting|CastToGameMode (Game|GetGameMode)))
        (Default|SpawnCharacters _asgame_mode (Class|GameplayStatics|GetPlayerControllerID (Game|GetPlayerController 1)))))))
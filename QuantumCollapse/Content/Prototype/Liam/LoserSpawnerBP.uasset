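; LoserSpawnerBP spawns the losing players as posed CS_Player characters, using loser data stored in NewGameInstance.
; On BeginPlay it loops over the stored LoserMeshes up to LosersNumber, spawning each at the matching LoserSpawns actor transform.
; Each spawn receives its stored mesh and material through WinningPlayerChanges, is set Static and loops a loss animation.
; The PlayerStart lookup result is unused, and an older PhysicsPlayer spawn path is disconnected.
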(event EventBeginPlay
  (bind _outactors (Actor|GetAllActorsOfClass "/Script/Engine.PlayerStart"))
  (Variables|Default|SetOut%20Actors _outactors)
  (bind _asnew_game_instance (Utilities|Casting|CastToNewGameInstance (Game|GetGameInstance)))
  (Variables|Default|Setgame%20instance _asnew_game_instance)
  (for (_ _array_index) (Variables|/Game/SideScrollerCPP/Blueprints/NewGameInstance.NewGameInstance_C|GetLoserMeshes (Variables|Default|Getgame%20instance))
    (if (<= _array_index (- (Variables|/Game/SideScrollerCPP/Blueprints/NewGameInstance.NewGameInstance_C|GetLosersNumber (Variables|Default|Getgame%20instance)) 1))
      (bind _returnvalue (Game|SpawnActorfromClass "/Game/Prototype/Liam/CS_Player.CS_Player_C" (Transformation|GetActorTransform (Utilities|Array|Get(acopy) (Variables|Default|GetLoserSpawns) _array_index)) "Undefined" 0 0 0))
      (Variables|Default|SetLoserCS _returnvalue)
      (Default|WinningPlayerChanges _returnvalue (Utilities|Array|Get(acopy) (Variables|/Game/SideScrollerCPP/Blueprints/NewGameInstance.NewGameInstance_C|GetLoserMeshes (Variables|Default|Getgame%20instance)) _array_index) (Utilities|Array|Get(acopy) (Variables|/Game/SideScrollerCPP/Blueprints/NewGameInstance.NewGameInstance_C|GetLoserMaterials (Variables|Default|Getgame%20instance)) _array_index))
      (Transformation|SetMobility (Variables|/Script/Engine.Actor|GetRootComponent (Variables|Default|GetLoserCS)) "Static")
      (Components|Animation|PlayAnimation (Variables|/Game/Prototype/Liam/CS_Player.CS_Player_C|GetSkeletalMesh _returnvalue) "/Game/Characters/Animations/Results_Screen/Anim_LossLoop.Anim_LossLoop" true))))

(fn ConstructionScript)
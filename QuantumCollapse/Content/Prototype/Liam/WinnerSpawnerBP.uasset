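; WinnerSpawnerBP is an actor that presents the match winner and handles the return to the main menu.
; On BeginPlay it spawns a CS_Player at its transform, applies the winner mesh and material from NewGameInstance, makes it static and loops a victory animation.
; Pressing Jump resets the game instance to defaults and opens DEV_MainMenu.
; A disconnected older path that spawns a PhysicsPlayer instead never runs.
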(event EventBeginPlay
  (bind _asnew_game_instance (Utilities|Casting|CastToNewGameInstance (Game|GetGameInstance)))
  (Variables|Default|Setgame%20instance _asnew_game_instance)
  (bind _returnvalue (Game|SpawnActorfromClass "/Game/Prototype/Liam/CS_Player.CS_Player_C" (Transformation|GetActorTransform) "Undefined" 0 0 0))
  (Variables|Default|SetCSPlayer _returnvalue)
  (Default|WinningPlayerChanges (Variables|Default|GetCSPlayer) (Variables|/Game/SideScrollerCPP/Blueprints/NewGameInstance.NewGameInstance_C|GetWinnerMesh (Variables|Default|Getgame%20instance)) (Variables|/Game/SideScrollerCPP/Blueprints/NewGameInstance.NewGameInstance_C|GetWinnerMaterial (Variables|Default|Getgame%20instance)))
  (Transformation|SetMobility (Variables|/Script/Engine.Actor|GetRootComponent (Variables|Default|GetCSPlayer)) "Static")
  (Components|Animation|PlayAnimation (Variables|/Game/Prototype/Liam/CS_Player.CS_Player_C|GetSkeletalMesh _returnvalue) "/Game/Characters/Animations/Results_Screen/Anim_VictoryLoop.Anim_VictoryLoop" true))

(event Input|ActionEvents|InputActionJump
  (params (Key :type Key%20Structure :default "None"))
  (:Pressed
    (Default|ResettoDefaultValues (Variables|Default|Getgame%20instance))
    (Game|OpenLevel(byName) "DEV_MainMenu")))

(fn ConstructionScript)
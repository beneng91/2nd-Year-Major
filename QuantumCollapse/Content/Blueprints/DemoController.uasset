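; Player controller for local multiplayer character select, where gamepad players join, cycle skins and materials, and ready up.
; BeginPlay hides the CS_Player pawns; joining possesses and reveals the one matching the controller ID.
; Choices and join/ready counts go to NewGameInstance, while per-player UI_PlayerSelect events fire on menu actors found by display name.
; Once player one readies, Tick moves their input to the CharacterSelect menu actor.
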(event Custom|P1%20Join
  (Class|WidgetSwitcher|SetActiveWidgetIndex (Variables|/Game/Widgets/Menu/Elements/UI_PlayerSelect_Base.UI_PlayerSelect_Base_C|GetJoinStatusSwitcher (Variables|Default|GetPlayer1Selector)) 1)
  (Default|OnActivate (Variables|Default|GetPlayer1Selector)))

(event EventBeginPlay
  ;[1 1 1] Hides all players at beginplay
  (bind _ascs_game_state_base (Utilities|Casting|CastToCS_GameStateBase (Game|GetGameState)))
  (for (_ _array_index) (Variables|/Game/Blueprints/CS_GameStateBase.CS_GameStateBase_C|GetCS_PlayerList _ascs_game_state_base)
    (Pawn|Possess self (Utilities|Array|Get(acopy) (Variables|/Game/Blueprints/CS_GameStateBase.CS_GameStateBase_C|GetCS_PlayerList _ascs_game_state_base) _array_index))
    (Rendering|SetActorHiddenInGame (Utilities|Array|Get(acopy) (Variables|/Game/Blueprints/CS_GameStateBase.CS_GameStateBase_C|GetCS_PlayerList _ascs_game_state_base) _array_index) true)))

(event EventTick
  (params (DeltaSeconds :type Float%20%28single-precision%29))
  (if (and (Variables|Default|GetisReadiedUp) (== (Class|GameplayStatics|GetPlayerControllerID self) 0))
    (Input|DisableInput (Game|GetPlayerController 0))
    (bind _outactors (Actor|GetAllActorsOfClass "/Game/Widgets/Menu/BP_Menu_Base.BP_Menu_Base_C"))
    (for _array_element _outactors
      (if (Variables|/Game/Widgets/Menu/BP_Menu_Base.BP_Menu_Base_C|GetCharacterSelect _array_element)
        (Input|EnableInput _array_element (Game|GetPlayerController 0))))))

(event Input|ActionEvents|InputActionChangeMaterialLeft
  (params (Key :type Key%20Structure :default "None"))
  (bind _self self)
  (bind _returnvalue (Class|GameplayStatics|GetPlayerControllerID _self))
  ;[1 1 1] material change
  (:Pressed
    (bind _asnew_game_instance (Utilities|Casting|CastToNewGameInstance (Game|GetGameInstance)))
    (bind _ascs_player (Utilities|Casting|CastToCS_Player (Game|Player|GetPlayerPawn _returnvalue)))
    (bind _result (Math|Integer|IncrementInt (Variables|/Game/Prototype/Liam/CS_Player.CS_Player_C|GetMaterialInstance _ascs_player))
      (:%20%20
        (Development|PrintString (Utilities|String|ToString(Integer) (Variables|/Game/Prototype/Liam/CS_Player.CS_Player_C|GetMaterialInstance _ascs_player)))
        (if (> _result (Variables|Default|GetMaxPlayerInt))
          (Variables|/Game/Prototype/Liam/CS_Player.CS_Player_C|SetMaterialInstance _ascs_player (Variables|Default|GetMinPlayerInt)))
        (switch int (Variables|/Game/Prototype/Liam/CS_Player.CS_Player_C|GetMeshInstance _ascs_player)
          (:0
            (Rendering|Material|SetMaterial (Variables|/Game/Prototype/Liam/CS_Player.CS_Player_C|GetSkeletalMesh _ascs_player) 0 (Utilities|Array|Get(acopy) (Variables|/Game/Prototype/Liam/CS_Player.CS_Player_C|GetMaterialInstancesArray _ascs_player) (Variables|/Game/Prototype/Liam/CS_Player.CS_Player_C|GetMaterialInstance _ascs_player)))
            (Utilities|Array|SetArrayElem (Variables|/Game/SideScrollerCPP/Blueprints/NewGameInstance.NewGameInstance_C|GetPlayerSelectedMaterialByInt _asnew_game_instance) _returnvalue 0))
          (:1
            (Rendering|Material|SetMaterial (Variables|/Game/Prototype/Liam/CS_Player.CS_Player_C|GetSkeletalMesh _ascs_player) 0 (Utilities|Array|Get(acopy) (Variables|/Game/Prototype/Liam/CS_Player.CS_Player_C|GetMaterialInstancesArrayOtter _ascs_player) (Variables|/Game/Prototype/Liam/CS_Player.CS_Player_C|GetMaterialInstance _ascs_player)))
            (Utilities|Array|SetArrayElem (Variables|/Game/SideScrollerCPP/Blueprints/NewGameInstance.NewGameInstance_C|GetPlayerSelectedMaterialByInt _asnew_game_instance) _returnvalue 0))
          (:2
            (Rendering|Material|SetMaterial (Variables|/Game/Prototype/Liam/CS_Player.CS_Player_C|GetSkeletalMesh _ascs_player) 0 (Utilities|Array|Get(acopy) (Variables|/Game/Prototype/Liam/CS_Player.CS_Player_C|GetMaterialInstancesArrayRetro _ascs_player) (Variables|/Game/Prototype/Liam/CS_Player.CS_Player_C|GetMaterialInstance _ascs_player)))
            (Utilities|Array|SetArrayElem (Variables|/Game/SideScrollerCPP/Blueprints/NewGameInstance.NewGameInstance_C|GetPlayerSelectedMaterialByInt _asnew_game_instance) _returnvalue 0))
          (:3
            (Rendering|Material|SetMaterial (Variables|/Game/Prototype/Liam/CS_Player.CS_Player_C|GetSkeletalMesh _ascs_player) 0 (Utilities|Array|Get(acopy) (Variables|/Game/Prototype/Liam/CS_Player.CS_Player_C|GetMaterialInstancesArraySinister _ascs_player) (Variables|/Game/Prototype/Liam/CS_Player.CS_Player_C|GetMaterialInstance _ascs_player)))
            (Utilities|Array|SetArrayElem (Variables|/Game/SideScrollerCPP/Blueprints/NewGameInstance.NewGameInstance_C|GetPlayerSelectedMaterialByInt _asnew_game_instance) _returnvalue 0)))
        (bind _outactors (Actor|GetAllActorsOfClass "/Game/Widgets/Menu/BP_Menu_Base.BP_Menu_Base_C"))
        (for _array_element _outactors
          (if (Utilities|String|Contains (Utilities|GetDisplayName _array_element) "PlayerSelect")
            (bind _asui_player_select (Utilities|Casting|CastToUI_PlayerSelect (UserInterface|GetWidget (Variables|/Game/Widgets/Menu/BP_Menu_Base.BP_Menu_Base_C|GetMenuWidget _array_element))))
            (switch int _returnvalue
              (:0
                (Default|P1Up _asui_player_select))
              (:1
                (Default|P2Up _asui_player_select))
              (:2
                (Default|P3Up _asui_player_select))
              (:3
                (Default|P4Up _asui_player_select)))))))))

(event Input|ActionEvents|InputActionChangeMaterialRight
  (params (Key :type Key%20Structure :default "None"))
  (bind _self self)
  (bind _returnvalue (Class|GameplayStatics|GetPlayerControllerID _self))
  ;[1 1 1] material change
  (:Pressed
    (bind _asnew_game_instance (Utilities|Casting|CastToNewGameInstance (Game|GetGameInstance)))
    (bind _ascs_player (Utilities|Casting|CastToCS_Player (Game|Player|GetPlayerPawn _returnvalue)))
    (bind _result (Math|Integer|DecrementInt (Variables|/Game/Prototype/Liam/CS_Player.CS_Player_C|GetMaterialInstance _ascs_player))
      (:%20%20
        (Development|PrintString (Utilities|String|ToString(Integer) (Variables|/Game/Prototype/Liam/CS_Player.CS_Player_C|GetMaterialInstance _ascs_player)))
        (if (< _result (Variables|Default|GetMinPlayerInt))
          (Variables|/Game/Prototype/Liam/CS_Player.CS_Player_C|SetMaterialInstance _ascs_player (Variables|Default|GetMaxPlayerInt)))
        (switch int (Variables|/Game/Prototype/Liam/CS_Player.CS_Player_C|GetMeshInstance _ascs_player)
          (:0
            (Rendering|Material|SetMaterial (Variables|/Game/Prototype/Liam/CS_Player.CS_Player_C|GetSkeletalMesh _ascs_player) 0 (Utilities|Array|Get(acopy) (Variables|/Game/Prototype/Liam/CS_Player.CS_Player_C|GetMaterialInstancesArray _ascs_player) (Variables|/Game/Prototype/Liam/CS_Player.CS_Player_C|GetMaterialInstance _ascs_player)))
            (Utilities|Array|SetArrayElem (Variables|/Game/SideScrollerCPP/Blueprints/NewGameInstance.NewGameInstance_C|GetPlayerSelectedMaterialByInt _asnew_game_instance) _returnvalue 0))
          (:1
            (Rendering|Material|SetMaterial (Variables|/Game/Prototype/Liam/CS_Player.CS_Player_C|GetSkeletalMesh _ascs_player) 0 (Utilities|Array|Get(acopy) (Variables|/Game/Prototype/Liam/CS_Player.CS_Player_C|GetMaterialInstancesArrayOtter _ascs_player) (Variables|/Game/Prototype/Liam/CS_Player.CS_Player_C|GetMaterialInstance _ascs_player)))
            (Utilities|Array|SetArrayElem (Variables|/Game/SideScrollerCPP/Blueprints/NewGameInstance.NewGameInstance_C|GetPlayerSelectedMaterialByInt _asnew_game_instance) _returnvalue 0))
          (:2
            (Rendering|Material|SetMaterial (Variables|/Game/Prototype/Liam/CS_Player.CS_Player_C|GetSkeletalMesh _ascs_player) 0 (Utilities|Array|Get(acopy) (Variables|/Game/Prototype/Liam/CS_Player.CS_Player_C|GetMaterialInstancesArrayRetro _ascs_player) (Variables|/Game/Prototype/Liam/CS_Player.CS_Player_C|GetMaterialInstance _ascs_player)))
            (Utilities|Array|SetArrayElem (Variables|/Game/SideScrollerCPP/Blueprints/NewGameInstance.NewGameInstance_C|GetPlayerSelectedMaterialByInt _asnew_game_instance) _returnvalue 0))
          (:3
            (Rendering|Material|SetMaterial (Variables|/Game/Prototype/Liam/CS_Player.CS_Player_C|GetSkeletalMesh _ascs_player) 0 (Utilities|Array|Get(acopy) (Variables|/Game/Prototype/Liam/CS_Player.CS_Player_C|GetMaterialInstancesArraySinister _ascs_player) (Variables|/Game/Prototype/Liam/CS_Player.CS_Player_C|GetMaterialInstance _ascs_player)))
            (Utilities|Array|SetArrayElem (Variables|/Game/SideScrollerCPP/Blueprints/NewGameInstance.NewGameInstance_C|GetPlayerSelectedMaterialByInt _asnew_game_instance) _returnvalue 0)))
        (bind _outactors (Actor|GetAllActorsOfClass "/Game/Widgets/Menu/BP_Menu_Base.BP_Menu_Base_C"))
        (for _array_element _outactors
          (if (Utilities|String|Contains (Utilities|GetDisplayName _array_element) "PlayerSelect")
            (bind _asui_player_select (Utilities|Casting|CastToUI_PlayerSelect (UserInterface|GetWidget (Variables|/Game/Widgets/Menu/BP_Menu_Base.BP_Menu_Base_C|GetMenuWidget _array_element))))
            (switch int _returnvalue
              (:0
                (Default|P1Down _asui_player_select))
              (:1
                (Default|P2Down _asui_player_select))
              (:2
                (Default|P3Down _asui_player_select))
              (:3
                (Default|P4Down _asui_player_select)))
            (else
              (Development|PrintString "failed not playerselect (material left)" true true "(R=0.000000,G=0.660000,B=1.000000,A=1.000000)" 1e+04))))))))

(event Input|ActionEvents|InputActionPauseGame
  (params (Key :type Key%20Structure :default "None"))
  ;[1 1 1] pause game
)

(event Input|ActionEvents|InputActionReadyUp
  (params (Key :type Key%20Structure :default "None"))
  (bind _self self)
  (bind _returnvalue (Class|GameplayStatics|GetPlayerControllerID _self))
  (:Pressed
    ;[1 1 1] original working
    (Variables|Default|SetReady true)
    (Development|PrintString "ready")
    (bind _ascs_player (Utilities|Casting|CastToCS_Player (Game|Player|GetPlayerPawn _returnvalue)))
    (CallFunction|ConfirmPlayerSelection _self _ascs_player _returnvalue)
    (bind _outactors (Actor|GetAllActorsOfClass "/Game/Widgets/Menu/BP_Menu_Base.BP_Menu_Base_C"))
    (for _array_element _outactors
      (if (Utilities|String|Contains (Utilities|GetDisplayName _array_element) "PlayerSelect")
        (bind _asui_player_select (Utilities|Casting|CastToUI_PlayerSelect (UserInterface|GetWidget (Variables|/Game/Widgets/Menu/BP_Menu_Base.BP_Menu_Base_C|GetMenuWidget _array_element))))
        (switch int _returnvalue
          (:0
            (Default|P1Confirm _asui_player_select))
          (:1
            (Default|P2Confirm _asui_player_select))
          (:2
            (Default|P3Confirm _asui_player_select))
          (:3
            (Default|P4Confirm _asui_player_select)))))))

(event Input|ActionEvents|InputActionChangeCharacterRight
  (params (Key :type Key%20Structure :default "None"))
  (bind _self self)
  (bind _returnvalue (Class|GameplayStatics|GetPlayerControllerID _self))
  ;[1 1 1] Cycling mesh
  (:Pressed
    (if (not (Variables|Default|GetisReadiedUp))
      (bind _ascs_player (Utilities|Casting|CastToCS_Player (Game|Player|GetPlayerPawn _returnvalue)))
      (bind _result (Math|Integer|DecrementInt (Variables|/Game/Prototype/Liam/CS_Player.CS_Player_C|GetMeshInstance _ascs_player))
        (:%20%20
          (if (< _result (Variables|Default|GetMinPlayerInt))
            (bind _output_get (Variables|/Game/Prototype/Liam/CS_Player.CS_Player_C|SetMeshInstance _ascs_player (Variables|Default|GetMaxPlayerInt)))
            (Class|SkinnedMeshComponent|SetSkeletalMesh (Variables|/Game/Prototype/Liam/CS_Player.CS_Player_C|GetSkeletalMesh _ascs_player) (Utilities|Array|Get(acopy) (Variables|/Game/Prototype/Liam/CS_Player.CS_Player_C|GetCharacterSkinArray _ascs_player) _output_get) true)
            (else
              (Class|SkinnedMeshComponent|SetSkeletalMesh (Variables|/Game/Prototype/Liam/CS_Player.CS_Player_C|GetSkeletalMesh _ascs_player) (Utilities|Array|Get(acopy) (Variables|/Game/Prototype/Liam/CS_Player.CS_Player_C|GetCharacterSkinArray _ascs_player) _result) true)))
          (switch int (Variables|/Game/Prototype/Liam/CS_Player.CS_Player_C|GetMeshInstance _ascs_player)
            (:0
              (Rendering|Material|SetMaterial (Variables|/Game/Prototype/Liam/CS_Player.CS_Player_C|GetSkeletalMesh _ascs_player) 0 (Utilities|Array|Get(acopy) (Variables|/Game/Prototype/Liam/CS_Player.CS_Player_C|GetMaterialInstancesArray _ascs_player) (Variables|/Game/Prototype/Liam/CS_Player.CS_Player_C|GetMeshInstance _ascs_player)))
              (Components|Animation|PlayAnimation (Variables|/Game/Prototype/Liam/CS_Player.CS_Player_C|GetSkeletalMesh _ascs_player) "/Game/Characters/Animations/CharacterSelect/Anim_MCIdle.Anim_MCIdle" true)
              (bind _outactors (Actor|GetAllActorsOfClass "/Game/Widgets/Menu/BP_Menu_Base.BP_Menu_Base_C" :!label _label))
              (for _array_element _outactors
                (if (Utilities|String|Contains (Utilities|GetDisplayName _array_element) "PlayerSelect")
                  (bind _asui_player_select (Utilities|Casting|CastToUI_PlayerSelect (UserInterface|GetWidget (Variables|/Game/Widgets/Menu/BP_Menu_Base.BP_Menu_Base_C|GetMenuWidget _array_element))))
                  (switch int _returnvalue
                    (:0
                      (Default|P1Right _asui_player_select))
                    (:1
                      (Default|P2Right _asui_player_select))
                    (:2
                      (Default|P3Right _asui_player_select))
                    (:3
                      (Default|P4Right _asui_player_select))))))
            (:1
              (Rendering|Material|SetMaterial (Variables|/Game/Prototype/Liam/CS_Player.CS_Player_C|GetSkeletalMesh _ascs_player) 0 (Utilities|Array|Get(acopy) (Variables|/Game/Prototype/Liam/CS_Player.CS_Player_C|GetMaterialInstancesArrayOtter _ascs_player) (Variables|/Game/Prototype/Liam/CS_Player.CS_Player_C|GetMeshInstance _ascs_player)))
              (Components|Animation|PlayAnimation (Variables|/Game/Prototype/Liam/CS_Player.CS_Player_C|GetSkeletalMesh _ascs_player) "/Game/Characters/Animations/CharacterSelect/Anim_OtterIdle.Anim_OtterIdle" true)
              (goto _label))
            (:2
              (Rendering|Material|SetMaterial (Variables|/Game/Prototype/Liam/CS_Player.CS_Player_C|GetSkeletalMesh _ascs_player) 0 (Utilities|Array|Get(acopy) (Variables|/Game/Prototype/Liam/CS_Player.CS_Player_C|GetMaterialInstancesArrayRetro _ascs_player) (Variables|/Game/Prototype/Liam/CS_Player.CS_Player_C|GetMeshInstance _ascs_player)))
              (Components|Animation|PlayAnimation (Variables|/Game/Prototype/Liam/CS_Player.CS_Player_C|GetSkeletalMesh _ascs_player) "/Game/Characters/Animations/CharacterSelect/Anim_RetroIdle.Anim_RetroIdle" true)
              (bind _outactors_2 (Actor|GetAllActorsOfClass "/Game/Widgets/Menu/BP_Menu_Base.BP_Menu_Base_C" :!label _label_2))
              (for _array_element_2 _outactors_2
                (if (Utilities|String|Contains (Utilities|GetDisplayName _array_element_2) "PlayerSelect")
                  (bind _asui_player_select_2 (Utilities|Casting|CastToUI_PlayerSelect (UserInterface|GetWidget (Variables|/Game/Widgets/Menu/BP_Menu_Base.BP_Menu_Base_C|GetMenuWidget _array_element_2))))
                  (switch int (Class|GameplayStatics|GetPlayerControllerID self)
                    (:0
                      (Default|P1Left _asui_player_select_2))
                    (:1
                      (Default|P2Left _asui_player_select_2))
                    (:2
                      (Default|P3Left _asui_player_select_2))
                    (:3
                      (Default|P4Left _asui_player_select_2))))))
            (:3
              (Rendering|Material|SetMaterial (Variables|/Game/Prototype/Liam/CS_Player.CS_Player_C|GetSkeletalMesh _ascs_player) 0 (Utilities|Array|Get(acopy) (Variables|/Game/Prototype/Liam/CS_Player.CS_Player_C|GetMaterialInstancesArraySinister _ascs_player) (Variables|/Game/Prototype/Liam/CS_Player.CS_Player_C|GetMeshInstance _ascs_player)))
              (Components|Animation|PlayAnimation (Variables|/Game/Prototype/Liam/CS_Player.CS_Player_C|GetSkeletalMesh _ascs_player) "/Game/Characters/Animations/CharacterSelect/Anim_SinisterIdle.Anim_SinisterIdle" true)
              (goto _label_2))))))))

(event Input|ActionEvents|InputActionChangeCharacterLeft
  (params (Key :type Key%20Structure :default "None"))
  (bind _self self)
  (bind _returnvalue (Class|GameplayStatics|GetPlayerControllerID _self))
  ;[1 1 1] Cycling mesh
  (:Pressed
    (if (not (Variables|Default|GetisReadiedUp))
      (bind _ascs_player (Utilities|Casting|CastToCS_Player (Game|Player|GetPlayerPawn _returnvalue)))
      (bind _result (Math|Integer|IncrementInt (Variables|/Game/Prototype/Liam/CS_Player.CS_Player_C|GetMeshInstance _ascs_player))
        (:%20%20
          (if (> _result (Variables|Default|GetMaxPlayerInt))
            (bind _output_get (Variables|/Game/Prototype/Liam/CS_Player.CS_Player_C|SetMeshInstance _ascs_player (Variables|Default|GetMinPlayerInt)))
            (Class|SkinnedMeshComponent|SetSkeletalMesh (Variables|/Game/Prototype/Liam/CS_Player.CS_Player_C|GetSkeletalMesh _ascs_player) (Utilities|Array|Get(acopy) (Variables|/Game/Prototype/Liam/CS_Player.CS_Player_C|GetCharacterSkinArray _ascs_player) _output_get) true)
            (else
              (Class|SkinnedMeshComponent|SetSkeletalMesh (Variables|/Game/Prototype/Liam/CS_Player.CS_Player_C|GetSkeletalMesh _ascs_player) (Utilities|Array|Get(acopy) (Variables|/Game/Prototype/Liam/CS_Player.CS_Player_C|GetCharacterSkinArray _ascs_player) _result) true)))
          (switch int (Variables|/Game/Prototype/Liam/CS_Player.CS_Player_C|GetMeshInstance (stale Input|ActionEvents|InputActionChangeCharacterRight _ascs_player))
            (:0
              (Rendering|Material|SetMaterial (Variables|/Game/Prototype/Liam/CS_Player.CS_Player_C|GetSkeletalMesh (stale Input|ActionEvents|InputActionChangeCharacterRight _ascs_player)) 0 (Utilities|Array|Get(acopy) (Variables|/Game/Prototype/Liam/CS_Player.CS_Player_C|GetMaterialInstancesArray (stale Input|ActionEvents|InputActionChangeCharacterRight _ascs_player)) (Variables|/Game/Prototype/Liam/CS_Player.CS_Player_C|GetMeshInstance (stale Input|ActionEvents|InputActionChangeCharacterRight _ascs_player))))
              (Components|Animation|PlayAnimation (Variables|/Game/Prototype/Liam/CS_Player.CS_Player_C|GetSkeletalMesh (stale Input|ActionEvents|InputActionChangeCharacterRight _ascs_player)) "/Game/Characters/Animations/CharacterSelect/Anim_MCIdle.Anim_MCIdle" true)
              (bind _outactors (Actor|GetAllActorsOfClass "/Game/Widgets/Menu/BP_Menu_Base.BP_Menu_Base_C" :!label _label))
              (for _array_element _outactors
                (if (Utilities|String|Contains (Utilities|GetDisplayName _array_element) "PlayerSelect")
                  (bind _asui_player_select (Utilities|Casting|CastToUI_PlayerSelect (UserInterface|GetWidget (Variables|/Game/Widgets/Menu/BP_Menu_Base.BP_Menu_Base_C|GetMenuWidget _array_element))))
                  (switch int (Class|GameplayStatics|GetPlayerControllerID self)
                    (:0
                      (Default|P1Right _asui_player_select))
                    (:1
                      (Default|P2Right _asui_player_select))
                    (:2
                      (Default|P3Right _asui_player_select))
                    (:3
                      (Default|P4Right _asui_player_select))))))
            (:1
              (Rendering|Material|SetMaterial (Variables|/Game/Prototype/Liam/CS_Player.CS_Player_C|GetSkeletalMesh (stale Input|ActionEvents|InputActionChangeCharacterRight _ascs_player)) 0 (Utilities|Array|Get(acopy) (Variables|/Game/Prototype/Liam/CS_Player.CS_Player_C|GetMaterialInstancesArrayOtter (stale Input|ActionEvents|InputActionChangeCharacterRight _ascs_player)) (Variables|/Game/Prototype/Liam/CS_Player.CS_Player_C|GetMeshInstance (stale Input|ActionEvents|InputActionChangeCharacterRight _ascs_player))))
              (Components|Animation|PlayAnimation (Variables|/Game/Prototype/Liam/CS_Player.CS_Player_C|GetSkeletalMesh (stale Input|ActionEvents|InputActionChangeCharacterRight _ascs_player)) "/Game/Characters/Animations/CharacterSelect/Anim_OtterIdle.Anim_OtterIdle" true)
              (goto _label))
            (:2
              (Rendering|Material|SetMaterial (Variables|/Game/Prototype/Liam/CS_Player.CS_Player_C|GetSkeletalMesh (stale Input|ActionEvents|InputActionChangeCharacterRight _ascs_player)) 0 (Utilities|Array|Get(acopy) (Variables|/Game/Prototype/Liam/CS_Player.CS_Player_C|GetMaterialInstancesArrayRetro (stale Input|ActionEvents|InputActionChangeCharacterRight _ascs_player)) (Variables|/Game/Prototype/Liam/CS_Player.CS_Player_C|GetMeshInstance (stale Input|ActionEvents|InputActionChangeCharacterRight _ascs_player))))
              (Components|Animation|PlayAnimation (Variables|/Game/Prototype/Liam/CS_Player.CS_Player_C|GetSkeletalMesh (stale Input|ActionEvents|InputActionChangeCharacterRight _ascs_player)) "/Game/Characters/Animations/CharacterSelect/Anim_RetroIdle.Anim_RetroIdle" true)
              (bind _outactors_2 (Actor|GetAllActorsOfClass "/Game/Widgets/Menu/BP_Menu_Base.BP_Menu_Base_C" :!label _label_2))
              (for _array_element_2 _outactors_2
                (if (Utilities|String|Contains (Utilities|GetDisplayName _array_element_2) "PlayerSelect")
                  (bind _asui_player_select_2 (Utilities|Casting|CastToUI_PlayerSelect (UserInterface|GetWidget (Variables|/Game/Widgets/Menu/BP_Menu_Base.BP_Menu_Base_C|GetMenuWidget _array_element_2))))
                  (switch int _returnvalue
                    (:0
                      (Default|P1Left _asui_player_select_2))
                    (:1
                      (Default|P2Left _asui_player_select_2))
                    (:2
                      (Default|P3Left _asui_player_select_2))
                    (:3
                      (Default|P4Left _asui_player_select_2))))))
            (:3
              (Rendering|Material|SetMaterial (Variables|/Game/Prototype/Liam/CS_Player.CS_Player_C|GetSkeletalMesh (stale Input|ActionEvents|InputActionChangeCharacterRight _ascs_player)) 0 (Utilities|Array|Get(acopy) (Variables|/Game/Prototype/Liam/CS_Player.CS_Player_C|GetMaterialInstancesArraySinister (stale Input|ActionEvents|InputActionChangeCharacterRight _ascs_player)) (Variables|/Game/Prototype/Liam/CS_Player.CS_Player_C|GetMeshInstance (stale Input|ActionEvents|InputActionChangeCharacterRight _ascs_player))))
              (Components|Animation|PlayAnimation (Variables|/Game/Prototype/Liam/CS_Player.CS_Player_C|GetSkeletalMesh (stale Input|ActionEvents|InputActionChangeCharacterRight _ascs_player)) "/Game/Characters/Animations/CharacterSelect/Anim_SinisterIdle.Anim_SinisterIdle" true)
              (goto _label_2))))))))

(event Input|ActionEvents|InputActionConnect
  (params (Key :type Key%20Structure :default "None"))
  (bind _self self)
  (bind _returnvalue (Class|GameplayStatics|GetPlayerControllerID _self))
  (:Pressed
    ;[1 1 1] Players can join game with any key
    (if (not (Variables|Default|GetPlayer%20Joined))
      (if (Variables|Default|GetCanUpdatePlayerCount)
        (if (Class|KismetInputLibrary|KeyIsGamepadKey Key)
          (Utilities|FlowControl|DoOnce false
            (:Completed
              ;[1 1 1] Spawns player in and possess character based on gamepad joined
              (bind _ascs_game_state_base (Utilities|Casting|CastToCS_GameStateBase (Game|GetGameState)))
              (bind _asnew_game_instance (Utilities|Casting|CastToNewGameInstance (Game|GetGameInstance)))
              (for _array_element (Variables|/Game/Blueprints/CS_GameStateBase.CS_GameStateBase_C|GetCS_PlayerList _ascs_game_state_base)
                (Pawn|Possess _self (Utilities|Array|Get(acopy) (Variables|/Game/Blueprints/CS_GameStateBase.CS_GameStateBase_C|GetCS_PlayerList _ascs_game_state_base) _returnvalue))
                (Rendering|SetActorHiddenInGame (Utilities|Array|Get(acopy) (Variables|/Game/Blueprints/CS_GameStateBase.CS_GameStateBase_C|GetCS_PlayerList _ascs_game_state_base) _returnvalue) false)
                (Components|Animation|PlayAnimation (Variables|/Game/Prototype/Liam/CS_Player.CS_Player_C|GetSkeletalMesh (Utilities|Array|Get(acopy) (Variables|/Game/Blueprints/CS_GameStateBase.CS_GameStateBase_C|GetCS_PlayerList _ascs_game_state_base) _returnvalue)) "/Game/Characters/Animations/CharacterSelect/Anim_MCIdle.Anim_MCIdle" false))
              (Math|Integer|IncrementInt (Variables|/Game/SideScrollerCPP/Blueprints/NewGameInstance.NewGameInstance_C|GetMaxPlayerCount _asnew_game_instance)
                (:%20%20
                  (Utilities|Array|SetArrayElem (Variables|/Game/SideScrollerCPP/Blueprints/NewGameInstance.NewGameInstance_C|GetPlayerSelectedMaterialByInt _asnew_game_instance) _returnvalue (Variables|/Game/Prototype/Liam/CS_Player.CS_Player_C|GetMaterialInstance (Utilities|Array|Get(acopy) (Variables|/Game/Blueprints/CS_GameStateBase.CS_GameStateBase_C|GetCS_PlayerList _ascs_game_state_base) _returnvalue)))
                  (bind _output_get (Variables|Default|SetPlayer%20Joined true))
                  (Development|PrintString "player joined" _output_get true "(R=0.959213,G=1.000000,B=0.000000,A=1.000000)" 1e+03)
                  (bind _outactors (Actor|GetAllActorsOfClass "/Game/Widgets/Menu/BP_Menu_Base.BP_Menu_Base_C"))
                  (for _array_element_2 _outactors
                    (if (Utilities|String|Contains (Utilities|GetDisplayName _array_element_2) "PlayerSelect")
                      (bind _asui_player_select (Utilities|Casting|CastToUI_PlayerSelect (UserInterface|GetWidget (Variables|/Game/Widgets/Menu/BP_Menu_Base.BP_Menu_Base_C|GetMenuWidget _array_element_2))))
                      (switch int _returnvalue
                        (:0
                          (Default|P1Join _asui_player_select))
                        (:1
                          (Default|P2Join _asui_player_select))
                        (:2
                          (Default|P3Join _asui_player_select))
                        (:3
                          (Default|P4Join _asui_player_select))))))))))))))

(fn ConstructionScript)

(fn ConfirmPlayerSelection
  (params (CS%20Player :type CS%20Player%20Object%20Reference%20%28by%20ref%29) (PlayerNumber :type Integer%20%28by%20ref%29))
  (bind _outactors (Actor|GetAllActorsOfClass "/Game/Prototype/Liam/CS_Player.CS_Player_C"))
  (bind _output_get (Variables|Default|SetcsPlayers _outactors))
  (bind _asnew_game_instance (Utilities|Casting|CastToNewGameInstance (Game|GetGameInstance)))
  (for (_ _array_index) _output_get
    (if (== _array_index PlayerNumber)
      (Utilities|Array|SetArrayElem (Variables|/Game/SideScrollerCPP/Blueprints/NewGameInstance.NewGameInstance_C|GetPlayerSelectedMeshByInt _asnew_game_instance) _array_index (Variables|/Game/Prototype/Liam/CS_Player.CS_Player_C|GetMeshInstance CS%20Player))
      (Utilities|Array|SetArrayElem (Variables|/Game/SideScrollerCPP/Blueprints/NewGameInstance.NewGameInstance_C|GetPlayerSelectedMaterialByInt _asnew_game_instance) _array_index (Variables|/Game/Prototype/Liam/CS_Player.CS_Player_C|GetMaterialInstance CS%20Player))
      (if (not (Variables|Default|GetisReadiedUp))
        (Variables|Default|SetisReadiedUp true)
        (Math|Integer|IncrementInt (Variables|/Game/SideScrollerCPP/Blueprints/NewGameInstance.NewGameInstance_C|GetreadyPlayers _asnew_game_instance))))))
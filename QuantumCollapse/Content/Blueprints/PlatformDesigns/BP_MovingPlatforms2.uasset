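; Moving platform actor that eases back and forth on a loop from BeginPlay, with a configurable destination, duration and pause.
; MoveStart and MoveReturn trigger each other through two MoveComponentTo nodes on PlatformHolder, with a delay between legs; MoveFreeze stops both moves.
; The construction script shows either a child-actor Blueprint or a static mesh with material and style overrides, then configures the point light.
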(event Custom|MoveReturn
  (Components|MoveComponentTo (Variables|Default|GetPlatform%20Holder) "0, 0, 0" "0, 0, 0" true true (Variables|PlatformControls|GetMovementDuration) false)
  (Utilities|FlowControl|Delay (Variables|PlatformControls|Getdelay))
  (CallFunction|MoveStart))

(event Custom|Move%20Freeze
  (Utilities|FlowControl|Sequence
    (:then_0
      (Components|MoveComponentTo (Variables|Default|GetPlatform%20Holder) (Variables|PlatformControls|GetMovementDestination) "0, 0, 0" true true (Variables|PlatformControls|GetMovementDuration) false) ; enters at Stop
    )
    (:then_1
      (Components|MoveComponentTo (Variables|Default|GetPlatform%20Holder) "0, 0, 0" "0, 0, 0" true true (Variables|PlatformControls|GetMovementDuration) false) ; enters at Stop
    )))

(event Custom|Move%20Start
  (Components|MoveComponentTo (Variables|Default|GetPlatform%20Holder) (Variables|PlatformControls|GetMovementDestination) "0, 0, 0" true true (Variables|PlatformControls|GetMovementDuration) false)
  (Utilities|FlowControl|Delay (Variables|PlatformControls|Getdelay))
  (CallFunction|MoveReturn))

(event EventBeginPlay
  ;[1 1 1] Begin Play
  (Variables|PlatformControls|SetmovementOrigin (Utilities|PlatformLocation))
  (CallFunction|MoveStart))

(fn ConstructionScript
  (if (Variables|PlatformControls|GetUseBP)
    (Rendering|SetVisibility (Variables|Default|GetPlatform) false false)
    (Rendering|SetVisibility (Variables|Default|GetBlueprintPlatform) true false)
    (ChildActorComponent|SetChildActorClass (Variables|Default|GetBlueprintPlatform) (Variables|PlatformControls|GetPlatformBP))
    (CallFunction|SetLighting)
    (else
      (Rendering|SetVisibility (Variables|Default|GetPlatform) true false)
      (Rendering|SetVisibility (Variables|Default|GetBlueprintPlatform) false false)
      (Components|StaticMesh|SetStaticMesh (Variables|Default|GetPlatform) (Variables|PlatformControls|GetPlatformMesh))
      (CallFunction|MaterialOverride (Actor|GetComponentsByClass "/Script/Engine.StaticMeshComponent") (Variables|MaterialOptions|GetMaterial) (Variables|MaterialOptions|GetDarken) (Variables|CelShadeOptions|GetCelShader) (Variables|CelShadeOptions|GetLineart) 0.0)
      (CallFunction|SetLighting))))

(fn SetLighting
  (bind _pointlight (Variables|Default|GetPointLight))
  (Rendering|Components|Light|SetIntensity _pointlight (Variables|Light|GetIntensity))
  (Rendering|Components|Light|SetLightColor _pointlight (Variables|Light|GetLight%20Colour) true)
  (Rendering|Lighting|SetAttenuationRadius _pointlight (Variables|Light|GetAttenuation%20Radius))
  (Class|LightComponent|SetTemperature _pointlight (Variables|Light|GetTemperature))
  (Class|LightComponent|SetUseTemperature _pointlight (Variables|Light|GetUse%20Temperature))
  (Transformation|AddWorldOffset _pointlight (+ (Variables|Light|GetPosition%20Offset) (Variables|/Script/Engine.SceneComponent|GetRelativeLocation (Variables|Default|GetPointLight))) false false))
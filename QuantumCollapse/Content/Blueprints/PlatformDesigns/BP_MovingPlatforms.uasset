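; Moving platform actor that travels between its placed position and an offset via an InterpToMovement component over a set duration.
; The construction script applies the chosen mesh, material override with darken, cel-shade and outline options, and point light settings.
; It rebuilds the movement's two absolute control points from the root's world location plus RelativeLocation.
; All setup happens at construction, and the event graph holds only disabled stub events.
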(event EventBeginPlay)

(event Collision|EventActorBeginOverlap
  (params (OtherActor :type Actor%20Object%20Reference)))

(event EventTick
  (params (DeltaSeconds :type Float%20%28single-precision%29)))

(fn ConstructionScript
  (bind _defaultsceneroot (Variables|Default|GetDefaultSceneRoot))
  (bind _returnvalue (Transformation|GetWorldLocation _defaultsceneroot))
  (Components|StaticMesh|SetStaticMesh (Variables|Default|GetPlatform) (Variables|PlatformControls|GetPlatformMesh))
  (CallFunction|MaterialOverride (Actor|GetComponentsByClass "/Script/Engine.StaticMeshComponent") (Variables|MaterialOptions|GetMaterial) (Variables|MaterialOptions|GetDarken) (Variables|CelShadeOptions|GetCelShader) (Variables|CelShadeOptions|GetLineart))
  (CallFunction|SetLighting)
  (Variables|/Script/Engine.InterpToMovementComponent|SetControlPoints (Variables|Default|GetInterpToMovement) (Utilities|Array|MakeArray (Utilities|Struct|MakeInterpControlPoint _returnvalue false) (Utilities|Struct|MakeInterpControlPoint (+ _returnvalue (Variables|PlatformControls|GetRelative%20Location)) false)))
  (Variables|/Script/Engine.InterpToMovementComponent|SetDuration (Variables|Default|GetInterpToMovement) (Variables|PlatformControls|GetDuration)))

(fn SetLighting
  (bind _pointlight (Variables|Default|GetPointLight))
  (Rendering|Components|Light|SetIntensity _pointlight (Variables|Light|GetIntensity))
  (Rendering|Components|Light|SetLightColor _pointlight (Variables|Light|GetLight%20Colour) true)
  (Rendering|Lighting|SetAttenuationRadius _pointlight (Variables|Light|GetAttenuation%20Radius))
  (Class|LightComponent|SetTemperature _pointlight (Variables|Light|GetTemperature))
  (Class|LightComponent|SetUseTemperature _pointlight (Variables|Light|GetUse%20Temperature))
  (Transformation|AddWorldOffset _pointlight (+ (Variables|Light|GetPosition%20Offset) (Variables|/Script/Engine.SceneComponent|GetRelativeLocation (Variables|Default|GetPointLight))) false false))
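; Floating warehouse platform that spawns a configurable platform Blueprint as a child actor and bobs it gently up and down.
; On BeginPlay it sets the child actor class and starts a self-repeating float loop.
; The Float Behaviour macro eases PlatformHandle up by a randomised, intensity-scaled height and back to its relative origin over random durations.
; The construction script applies dark, cel-shaded and outline material options to its static meshes.
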(event Custom|FloatStart
  (Utilities|FloatBehaviour
    (:ExecOut
      (CallFunction|FloatStart))))

(event EventBeginPlay
  (if true
    (ChildActorComponent|SetChildActorClass (Variables|Default|GetPlatform) (Variables|Default|GetPlatformBlueprint))
    (Utilities|FloatBehaviour
      (:ExecOut
        (CallFunction|FloatStart)))))

(fn ConstructionScript
  (CallFunction|MaterialOverride (Actor|GetComponentsByClass "/Script/Engine.StaticMeshComponent") 0 (Variables|Default|GetIs%20Dark) (Variables|Default|GetIs%20Cel%20Shaded) (Variables|Default|GetIs%20Outlined) 0.0))
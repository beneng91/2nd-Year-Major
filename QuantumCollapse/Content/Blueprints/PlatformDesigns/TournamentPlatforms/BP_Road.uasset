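; BP_Road is a road piece for tournament platforms whose look can be customised per instance.
; Its construction script creates a dynamic instance of the EnvSDRoad component's first material and reapplies it.
; When Darken is set, it dims the colour multiplier and sets the emissive colour from Colour; otherwise it uses full brightness.
; The event graph holds only disabled stub events, so there is no runtime logic.
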(event EventBeginPlay)

(event Collision|EventActorBeginOverlap
  (params (OtherActor :type Actor%20Object%20Reference)))

(event EventTick
  (params (DeltaSeconds :type Float%20%28single-precision%29)))

(fn ConstructionScript
  (bind _env_sd_road (Variables|Default|GetEnv_SD_Road))
  (bind _returnvalue (Rendering|Material|CreateDynamicMaterialInstance _env_sd_road 0 (Rendering|Material|GetMaterial _env_sd_road 0) "CustomRoad" :!class /Script/Engine.PrimitiveComponent))
  (LocalVariables|Set_dynamicMaterial _returnvalue)
  (if (Variables|Default|GetDarken)
    (Rendering|Material|SetScalarParameterValue (LocalVariables|Get_dynamicMaterial) "ColourMultiplier" 0.4 :!class /Script/Engine.MaterialInstanceDynamic)
    (Rendering|Material|SetVectorParameterValue (LocalVariables|Get_dynamicMaterial) "EmissiveColour" (LocalVariables|Get_colour) :!class /Script/Engine.MaterialInstanceDynamic)
    (else
      (Rendering|Material|SetScalarParameterValue (LocalVariables|Get_dynamicMaterial) "ColourMultiplier" 1.0 :!class /Script/Engine.MaterialInstanceDynamic)))
  (Rendering|Material|SetMaterial (Variables|Default|GetEnv_SD_Road) 0 (LocalVariables|Get_dynamicMaterial)))
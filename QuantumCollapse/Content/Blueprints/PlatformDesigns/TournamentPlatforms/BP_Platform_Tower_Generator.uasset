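; Procedural tournament platform tower that assembles itself in the construction script from a configurable number of extra stacked mesh segments.
; TowerGenerator adds tagged segments at fixed height steps above the base piece, plus an optional capping mesh that can be mirrored.
; RenderingDetails then passes all static meshes to a MaterialOverride call for material, darkening, cel-shading, outline and brightness settings.
; A local MaterialOverrides function with similar custom-depth and dynamic-material logic is not called here.
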(event EventBeginPlay)

(event Collision|EventActorBeginOverlap
  (params (OtherActor :type Actor%20Object%20Reference)))

(event EventTick
  (params (DeltaSeconds :type Float%20%28single-precision%29)))

(fn ConstructionScript
  (CallFunction|TowerGenerator)
  (CallFunction|RenderingDetails))

(fn TowerGenerator
  (bind _env_pf_small (Variables|Default|GetEnv_Pf_Small))
  (bind _relativerotation (Variables|/Script/Engine.SceneComponent|GetRelativeRotation _env_pf_small))
  (for _index (range 1 (Variables|TowerGeneration|GetExtra%20Towers))
    (bind _returnvalue (AddComponent|AddStaticMeshComponent false (Math|Transform|MakeTransform (+ (Variables|/Script/Engine.SceneComponent|GetRelativeLocation _env_pf_small) (* "0, 0,240.000000" _index)) _relativerotation)))
    (Variables|/Script/Engine.ActorComponent|SetComponentTags _returnvalue (Variables|Default|GetTags_0)))
  (if (Variables|TowerGeneration|GetAdd%20Capping?)
    (if (Variables|TowerGeneration|GetFlip%20Capping?)
      (bind _returnvalue_2 (AddComponent|AddStaticMeshComponent false (Math|Transform|MakeTransform (* "0, 0,240.000000" _index) _relativerotation "-1.000000,1,1")))
      (else
        (AddComponent|AddStaticMeshComponent false (Math|Transform|MakeTransform (* "0, 0,240.000000" _index) _relativerotation))))
    (Variables|/Script/Engine.ActorComponent|SetComponentTags _returnvalue_2 (Variables|Default|GetTags_0))))

(fn MaterialOverrides
  (for _array_element (Actor|GetComponentsByClass "/Script/Engine.StaticMeshComponent")
    (Rendering|SetRenderCustomDepth _array_element (Variables|CelShadeOptions|GetCel%20Shaded))
    (if (Variables|MaterialOverride|GetDarken)
      (bind _returnvalue (Rendering|Material|CreateDynamicMaterialInstance (Variables|MaterialOverride|GetMaterial) "Dark Material" "None" :!class /Script/Engine.KismetMaterialLibrary))
      (Rendering|Material|SetScalarParameterValue _returnvalue "ColourMultiplier" 0.75 :!class /Script/Engine.MaterialInstanceDynamic)
      (Rendering|Material|SetScalarParameterValue _returnvalue "EmissionBaseMultiplier" 0.1 :!class /Script/Engine.MaterialInstanceDynamic)
      (Rendering|Material|SetMaterial _array_element 0 _returnvalue)
      (else
        (Rendering|Material|SetMaterial _array_element 0 (Variables|MaterialOverride|GetMaterial))))
    (if (Variables|CelShadeOptions|GetLineart)
      (Rendering|SetCustomDepthStencilValue _array_element 3)
      (else
        (Rendering|SetCustomDepthStencilValue _array_element 0)))))

(fn RenderingDetails
  (CallFunction|MaterialOverride (Actor|GetComponentsByClass "/Script/Engine.StaticMeshComponent") (Variables|MaterialOverride|GetMaterial) (Variables|MaterialOverride|GetDarken) (Variables|CelShadeOptions|GetCel%20Shaded) (Variables|CelShadeOptions|GetLineart) (Variables|MaterialOverride|GetBrightness%20Multiplier)))
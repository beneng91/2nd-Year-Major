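; BP_skybox is a skybox actor that applies a configurable material to its sky mesh.
; The construction script calls SetSkyboxMaterial, which creates a dynamic instance of SkyboxMaterial on the mesh's first slot and stores it.
; It copies the Star, Power, Scene and Colour variables into scalar parameters, then assigns the instance to the mesh.
; All work happens at construction, as the event graph holds only disabled placeholder events.
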(event EventBeginPlay)

(event Collision|EventActorBeginOverlap
  (params (OtherActor :type Actor%20Object%20Reference)))

(event EventTick
  (params (DeltaSeconds :type Float%20%28single-precision%29)))

(fn ConstructionScript
  (CallFunction|SetSkyboxMaterial (Variables|Default|GetSkyBoxMesh)))

(fn SetSkyboxMaterial
  (params (SkyboxMesh :type Static%20Mesh%20Component%20Object%20Reference))
  (bind _returnvalue (Rendering|Material|CreateDynamicMaterialInstance SkyboxMesh 0 (Variables|SkyboxSettings|GetSkybox%20Material) "SkyboxInstance" :!class /Script/Engine.PrimitiveComponent))
  (bind _output_get (LocalVariables|SetInstancedSkyboxMat _returnvalue))
  (Rendering|Material|SetScalarParameterValue _output_get "Star" (Variables|SkyboxSettings|GetStar) :!class /Script/Engine.MaterialInstanceDynamic)
  (Rendering|Material|SetScalarParameterValue (LocalVariables|GetInstancedSkyboxMat) "Power" (Variables|SkyboxSettings|GetPower) :!class /Script/Engine.MaterialInstanceDynamic)
  (Rendering|Material|SetScalarParameterValue (LocalVariables|GetInstancedSkyboxMat) "Scene" (Variables|SkyboxSettings|GetScene) :!class /Script/Engine.MaterialInstanceDynamic)
  (Rendering|Material|SetScalarParameterValue (LocalVariables|GetInstancedSkyboxMat) "colour" (Variables|SkyboxSettings|GetColour) :!class /Script/Engine.MaterialInstanceDynamic)
  (Rendering|Material|SetMaterial (Variables|Default|GetSkyBoxMesh) 0 (LocalVariables|GetInstancedSkyboxMat)))